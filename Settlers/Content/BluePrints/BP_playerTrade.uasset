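; Player trade actor that holds one resource-card trade offer from the game manager's current player to other players.
; Sending and receiving maps count cards per type, and a valid trade needs both non-empty with no shared type.
; Receivers are queued and accept or deny, with AutoDeny rejecting those who fail the resource check.
; FinaliseTrade picks the final receiver, and MoveItems swaps the cards through PayPlayer calls in both directions.
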(event `/Game/Interfaces/I_tradeInterface.addItemToReceiving`
  (params (resourceCard :type "/Game/Data/E_resourceType Enum" :default "NewEnumerator7"))
  (`self.addItemToReceiving_` resourceCard))

(event `/Game/Interfaces/I_tradeInterface.addItemToSending`
  (params (resourceCard :type "/Game/Data/E_resourceType Enum" :default "NewEnumerator7"))
  (`self.addItemToSending_` resourceCard))

(event `/Game/Interfaces/I_tradeInterface.moveItems`
  (`self.moveItems_`))

(event `/Game/Interfaces/I_tradeInterface.removeItemFromReceiving`
  (params (resourceCard :type "/Game/Data/E_resourceType Enum" :default "NewEnumerator7"))
  (`self.removeItemFromReceiving_` resourceCard))

(event `/Game/Interfaces/I_tradeInterface.removeItemFromSending`
  (params (resourceCard :type "/Game/Data/E_resourceType Enum" :default "NewEnumerator7"))
  (`self.removeItemFromSending_` resourceCard))

(fn `acceptOffer`
  (params (accepter :type "/Game/BluePrints/BP_player Object Reference"))
  (`KismetArrayLibrary.Array_Add` (`self.acceptedPlayers`) accepter))

(fn `addItemToReceiving_`
  (params (resourceCard :type "/Game/Data/E_resourceType Enum" :default "NewEnumerator7"))
  (bind _receivingitems (`self.receivingItems`))
  (`BlueprintMapLibrary.Map_Add` _receivingitems resourceCard (+ (`BlueprintMapLibrary.Map_Find` _receivingitems resourceCard) 1)))

(fn `addItemToSending_`
  (params (resourceCard :type "/Game/Data/E_resourceType Enum" :default "NewEnumerator7"))
  (bind _sendingitems (`self.sendingItems`))
  (`BlueprintMapLibrary.Map_Add` _sendingitems resourceCard (+ (`BlueprintMapLibrary.Map_Find` _sendingitems resourceCard) 1)))

(fn `autoDeny`
  (for _array_element (`self.offerReceivers`)
    (bind _checksucceeded_ (`/Game/BluePrints/BP_player.checkResources` _array_element (`self.receivingItems`)))
    (if (not _checksucceeded_)
      (`self.denyOffer` _array_element))))

(fn `canReceiverIncreaseResource`
  (params (resourceCard :type "/Game/Data/E_resourceType Enum" :default "NewEnumerator7"))
  (returns (canIncrease :type Boolean))
  (return true))

(fn `canSenderIncreaseResource`
  (params (resourceCard :type "/Game/Data/E_resourceType Enum" :default "NewEnumerator7"))
  (returns (canIncrease :type Boolean))
  (return (< (`BlueprintMapLibrary.Map_Find` (`self.sendingItems`) resourceCard) (`BlueprintMapLibrary.Map_Find` (`.resourceCards_6_629E6944473B44BFE5C01789E3CC3565` (break `/Game/Data/S_Hand` (`/Game/BluePrints/BP_player.hand` (`self.sender`)))) resourceCard))))

(fn `denyOffer`
  (params (denier :type "/Game/BluePrints/BP_player Object Reference"))
  (`BlueprintSetLibrary.Set_Add` (`self.deniedPlayers`) denier)
  (`KismetArrayLibrary.Array_RemoveItem` (`self.offerReceivers`) denier))

(fn `finaliseTrade`
  (params (selectedPlayer :type "/Game/BluePrints/BP_player Object Reference"))
  (set `self.finalReceiver` selectedPlayer))

(fn `getNextOfferReceiver`
  (returns (player :type "/Game/BluePrints/BP_player Object Reference"))
  (locals (nextOfferReceiver :type "/Game/BluePrints/BP_player Object Reference"))
  (set `local.nextOfferReceiver` (`|GetArrayItem` (`self.offerReceivers`)))
  (`KismetArrayLibrary.Array_Remove` (`self.offerReceivers`))
  (return (`local.nextOfferReceiver`)))

(fn `getSender`
  (returns (sender :type "/Game/BluePrints/BP_player Object Reference"))
  (return (`self.sender`)))

(fn `includePlayer`
  (params (playerToInclude :type "/Game/BluePrints/BP_player Object Reference"))
  (`KismetArrayLibrary.Array_Add` (`self.offerReceivers`) playerToInclude)
  (`KismetSystemLibrary.PrintString` (`|GetEnumeratorNameAsString` (`/Game/BluePrints/BP_player.colour` playerToInclude))))

(fn `isTradeValid`
  (returns (valid :type Boolean))
  (bind _valid (`self.isTradeValid_`))
  (return _valid))

(fn `isTradeValid_`
  (returns (valid :type Boolean))
  ;[1 1 1] if either item map is empty
  (if (or (`BlueprintMapLibrary.Map_IsEmpty` (`self.sendingItems`)) (`BlueprintMapLibrary.Map_IsEmpty` (`self.receivingItems`)))
    (return false)
    (else
      ;[1 1 1] Check if a resource appears in both sendingItems and receivingItems - if it does return false
      (bind _keys (`BlueprintMapLibrary.Map_Keys` (`self.sendingItems`)))
      (bind _keys_2 (`BlueprintMapLibrary.Map_Keys` (`self.receivingItems`)))
      (for _array_element _keys_2
        (if (`KismetArrayLibrary.Array_Contains` _keys _array_element)
          (return false)))
      (return true))))

(fn `moveItems_`
  (bind _sender (`self.sender`))
  (bind _finalreceiver (`self.finalReceiver`))
  (`/Game/BluePrints/BP_player.payPlayer` _sender (`self.sendingItems`) _finalreceiver)
  (`/Game/BluePrints/BP_player.payPlayer` _finalreceiver (`self.receivingItems`) _sender)
  ;[1 0.05003 0.1098] Placeholder for log
  (`KismetSystemLibrary.PrintString` "trade complete "))

(fn `offerReceiversToString`
  (returns (offerReceivers :type String))
  (locals (offerReceiversString :type String))
  (for _array_element (`self.offerReceivers`)
    (set `local.offerReceiversString` (`KismetStringLibrary.Concat_StrStr` (`KismetStringLibrary.Concat_StrStr` (`local.offerReceiversString`) " ") (`|GetEnumeratorNameAsString` (`/Game/BluePrints/BP_player.colour` _array_element)))))
  (return (`local.offerReceiversString`)))

(fn `playerInOfferReceivers`
  (params (player :type "/Game/BluePrints/BP_player Object Reference"))
  (returns (playerIncluded :type Boolean))
  (return (`KismetArrayLibrary.Array_Contains` (`self.offerReceivers`) player)))

(fn `removeItemFromReceiving_`
  (params (resourceCard :type "/Game/Data/E_resourceType Enum" :default "NewEnumerator7"))
  (bind _receivingitems (`self.receivingItems`))
  (bind _value (`BlueprintMapLibrary.Map_Find` _receivingitems resourceCard))
  (if (== _value 0)
    (`KismetSystemLibrary.PrintString` "No more of this card type can be removed" true true (struct :`R` 0.761128 :`G` 0.60198 :`B` 1.0 :`A` 1.0))
    (else
      (`BlueprintMapLibrary.Map_Add` _receivingitems resourceCard (- _value 1)))))

(fn `removeItemFromSending_`
  (params (resourceCard :type "/Game/Data/E_resourceType Enum" :default "NewEnumerator7"))
  (bind _sendingitems (`self.sendingItems`))
  (bind _value (`BlueprintMapLibrary.Map_Find` _sendingitems resourceCard))
  (if (== _value 0)
    (`KismetSystemLibrary.PrintString` "No more of this card type can be removed" true true (struct :`R` 0.761128 :`G` 0.60198 :`B` 1.0 :`A` 1.0))
    (else
      (`BlueprintMapLibrary.Map_Add` _sendingitems resourceCard (- _value 1)))))

(fn `removePlayer`
  (params (playerToRemove :type "/Game/BluePrints/BP_player Object Reference"))
  (`KismetArrayLibrary.Array_RemoveItem` (`self.offerReceivers`) playerToRemove)
  (`KismetSystemLibrary.PrintString` (`|GetEnumeratorNameAsString` (`/Game/BluePrints/BP_player.colour` playerToRemove))))

(fn `tradeHasReceivers`
  (returns (hasReceivers :type Boolean))
  (if (`KismetArrayLibrary.Array_IsEmpty` (`self.offerReceivers`))
    (return false)
    (else
      (return true))))

(fn `UserConstructionScript`
  (bind _returnvalue (`GameplayStatics.GetActorOfClass` "/Game/BluePrints/BP_gameManager.BP_gameManager_C"))
  (bind _output_get (set `self.gameManger` _returnvalue))
  (set `self.sender` (`/Game/BluePrints/BP_gameManager.currentPlayer` _output_get)))