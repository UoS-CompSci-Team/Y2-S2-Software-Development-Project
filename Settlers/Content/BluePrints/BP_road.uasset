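; BP_road is a road slot between two settlement nodes on a board, storing its owning player.
; CanPlayerBuildRoad accepts an unowned slot if the player owns either end node or an adjacent road through an unoccupied shared node.
; On GameManager state updates, owned roads are shown, while unowned ones hide unless the current player can build there in one specific state.
; SetVisualColour assigns the owner and applies that player's colour material to the plane.
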(event `self.ReceiveBeginPlay`
  ;[1 1 1] initialise
  (`KismetSystemLibrary.Delay` 0.2)
  (add `/Game/BluePrints/BP_gameManager.gameStateUpdate` (`self.gameManager`) (delegate `gameStateUpdate`)))

(event `gameStateUpdate`
  ;[1 1 1] initialise
  (`self.gameStateUpdate_Process`))

(event `gameStateUpdate_Process`
  (bind _gamemanager (`self.gameManager`))
  ;[1 1 1] Update visibility on game state update
  (`KismetSystemLibrary.DelayUntilNextTick`)
  (if (`KismetSystemLibrary.IsValid` (`self.roadOwner`))
    (`SceneComponent.SetVisibility` (`self.Plane`) true false)
    (else
      (bind _canbuild (`self.canPlayerBuildRoad` (`/Game/BluePrints/BP_gameManager.currentPlayer` _gamemanager)))
      (if (not (and _canbuild (`|EnumEquality` (`/Game/BluePrints/BP_gameManager.gameState` _gamemanager) "NewEnumerator5")))
        (`SceneComponent.SetVisibility` (`self.Plane`) false false)))))

(fn `canPlayerBuildRoad`
  (params (playerChecking :type "/Game/BluePrints/BP_player Object Reference"))
  (returns (canBuild :type Boolean))
  (locals (totalAdjacentRods :type "Array of /Game/BluePrints/BP_road Object Reference") (numberOfAdjacentRoads :type Integer))
  (bind _nodea (`self.nodeA`))
  (bind _nodeb (`self.nodeB`))
  (bind _totaladjacentrods (`local.totalAdjacentRods`))
  ;[1 1 1] returns false if road is already built upon
  (bind _isbuiltupon (`self.isBuiltUpon`))
  (if _isbuiltupon
    (return false)
    (else
      ;[1 1 1] returns true if either adjacent settlement is owned by the checking player
      (if (or (== (`/Game/BluePrints/BP_settlementNode.player` _nodea) playerChecking) (== playerChecking (`/Game/BluePrints/BP_settlementNode.player` _nodeb)))
        (return true)
        (else
          ;[1 1 1] Checks if any roads adjacent to node A/B are owned by the player, returns true if more than one is found
          (`KismetArrayLibrary.Array_Append` _totaladjacentrods (`/Game/BluePrints/BP_settlementNode.adjacentRoads` _nodea))
          (`KismetArrayLibrary.Array_Append` _totaladjacentrods (`/Game/BluePrints/BP_settlementNode.adjacentRoads` _nodeb))
          (for _array_element (`local.totalAdjacentRods`)
            (if (== playerChecking (`/Game/BluePrints/BP_road.roadOwner` _array_element))
              (bind _nodea_2 (`/Game/BluePrints/BP_road.nodeA` _array_element))
              (if (or (== (`self.nodeA`) _nodea_2) (== _nodea_2 (`self.nodeB`)))
                (if (not (`KismetSystemLibrary.IsValid` (`/Game/BluePrints/BP_settlementNode.player` _nodea_2)))
                  (bind _output_get (set `local.numberOfAdjacentRoads` (+ 1 (`local.numberOfAdjacentRoads`)) :!label _label))
                  (if (> _output_get 0)
                    (break)))
                (elif (not (`KismetSystemLibrary.IsValid` (`/Game/BluePrints/BP_settlementNode.player` (`/Game/BluePrints/BP_road.nodeB` _array_element))))
                  (goto _label)))))
          (if (> (`local.numberOfAdjacentRoads`) 0)
            (return true)
            (else
              (return false))))))))

(fn `getOtherNode`
  (params (Node :type "/Game/BluePrints/BP_settlementNode Object Reference"))
  (returns (otherNode :type "/Game/BluePrints/BP_settlementNode Object Reference"))
  (if (== Node (`self.nodeA`))
    (return (`self.nodeB`))
    (else
      (return (`self.nodeA`)))))

(fn `isBuiltUpon`
  (returns (isBuiltUpon :type Boolean))
  (if (`KismetSystemLibrary.IsValid` (`self.roadOwner`))
    (return true)
    (else
      (return false))))

(fn `setVisualColour`
  (params (player :type "/Game/BluePrints/BP_player Object Reference"))
  (bind _plane (`self.Plane`))
  (set `self.roadOwner` player)
  (bind _output_get (set `self.colour` (`/Game/BluePrints/BP_player.colour` player)))
  (switch `/Game/Data/E_playerColours` _output_get
    (:`NewEnumerator0`
      (`PrimitiveComponent.SetMaterial` _plane 0 "/Game/Materials/M_baseRed.M_baseRed"))
    (:`NewEnumerator1`
      (`PrimitiveComponent.SetMaterial` _plane 0 "/Game/Materials/M_baseBlue.M_baseBlue"))
    (:`NewEnumerator2`
      (`PrimitiveComponent.SetMaterial` _plane 0 "/Game/Materials/M_baseGreen.M_baseGreen"))
    (:`NewEnumerator3`
      (`PrimitiveComponent.SetMaterial` _plane 0 "/Game/Materials/M_baseYellow.M_baseYellow"))))

(fn `UserConstructionScript`)