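; In-game unit test actor for a Catan-style board game, reporting failures as red on-screen messages.
; When RUNUNITTESTS is set, BeginPlay waits a second to avoid a crash, runs the suite, then quits.
; It validates road/settlement/hex links, player hands and robber movement and blocking, simulating rolls and clicks through debug functions.
; A settlement placement test exists but RunAllUnitTests does not call it.
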(event `self.ReceiveBeginPlay`
  (if (`self.RUN_UNIT_TESTS`)
    (bind _returnvalue (`GameplayStatics.GetActorOfClass` "/Game/BluePrints/BP_gameManager.BP_gameManager_C"))
    (set `self.gameManagerRef` _returnvalue)
    (`KismetSystemLibrary.Delay` 1.0) ; without delay, game crashes
    (`self.runAllUnitTests`)
    (`KismetSystemLibrary.QuitGame` null "Quit")))

(fn `runAllUnitTests`
  (`self.unitTestMapObjects`)
  (`self.unitTestPlayer`)
  (`self.unitTestRobber`))

(fn `Unit Test Settlement Placement`
  (locals (selectedSettlementNode :type "/Game/BluePrints/BP_settlementNode Object Reference") (iteratorNode :type "/Game/BluePrints/BP_settlementNode Object Reference"))
  (bind _selectedsettlementnode (`local.selectedSettlementNode`))
  (bind _selectedsettlementnode_2 (`local.selectedSettlementNode`))
  (bind _gamemanagerref (`self.gameManagerRef`))
  (bind _selectedsettlementnode_3 (`local.selectedSettlementNode`))
  (bind _selectedsettlementnode_4 (`local.selectedSettlementNode`))
  (bind _currentplayer (`/Game/BluePrints/BP_gameManager.currentPlayer` (`self.gameManagerRef`)))
  (bind _colour (`/Game/BluePrints/BP_settlementNode.colour` _selectedsettlementnode_2))
  (bind _currentplayer_2 (`/Game/BluePrints/BP_gameManager.currentPlayer` (`self.gameManagerRef`)))
  (bind _clickstate (`/Game/BluePrints/BP_gameManager.clickState` (`self.gameManagerRef`)))
  (bind _benableclickevents (`PlayerController.bEnableClickEvents` (`GameplayStatics.GetPlayerController` 0)))
  (bind _clickstate_2 (`/Game/BluePrints/BP_gameManager.clickState` (`self.gameManagerRef`)))
  (bind _benableclickevents_2 (`PlayerController.bEnableClickEvents` (`GameplayStatics.GetPlayerController` 0)))
  (bind _currentplayer_3 (`/Game/BluePrints/BP_gameManager.currentPlayer` (`self.gameManagerRef`)))
  (bind _colour_2 (`/Game/BluePrints/BP_player.colour` _currentplayer))
  ;[1 1 1] variable setup
  (set `/Game/BluePrints/BP_gameManager.snakeTurnsIndex` 1 (`self.gameManagerRef`)) ; testing with snake turns enabled (later disabled)
  (`/Game/BluePrints/BP_gameManager.Debug Make Settlements Clickable` _gamemanagerref)
  (bind _output_get (set `local.selectedSettlementNode` (`KismetArrayLibrary.Array_Random` (`/Game/BluePrints/BP_gameManager.settlementsNodes` _gamemanagerref))))
  (if (`|EnumEquality` (`/Game/BluePrints/BP_settlementNode.colour` _output_get) (`/Game/BluePrints/BP_player.colour` (`/Game/BluePrints/BP_gameManager.currentPlayer` (`self.gameManagerRef`))))
    (set `/Game/BluePrints/BP_settlementNode.colour` "NewEnumerator1" (`local.selectedSettlementNode`)) ; change settlement colour
  )
  ;[1 1 1] test if owner-less settlement nodes become visible when placing a settlement
  (for _array_element (`/Game/BluePrints/BP_gameManager.settlementsNodes` (`self.gameManagerRef`))
    (if (not (`SceneComponent.IsVisible` (`/Game/BluePrints/BP_settlementNode.Sphere` _array_element)))
      (`KismetSystemLibrary.PrintString` (`KismetStringLibrary.Concat_StrStr` "ERROR: not all spheres appeared when settlement placing function called and no settlements are owned. \nOne such node is \"" (`KismetSystemLibrary.GetDisplayName` _array_element) "\".") true true (struct :`R` 1.0 :`A` 1.0) 10.0)
      (break)))
  ;[1 1 1] test if settlement clicking is enabled
  (if (or (`|EnumInequality` _clickstate "NewEnumerator0") (not _benableclickevents))
    (`KismetSystemLibrary.PrintString` (`KismetStringLibrary.Concat_StrStr` "ERROR: settlements should be placable but user click events are disabled. \nClick state is \"" (`|GetEnumeratorNameAsString` _clickstate) "\" and click events enabled is \"" (`KismetStringLibrary.Conv_BoolToString` _benableclickevents) "\".") true true (struct :`R` 1.0 :`A` 1.0) 10.0))
  ;[1 1 1] click selected node
  (`/Game/BluePrints/BP_settlementNode.Debug Clicked(Sphere)` (`local.selectedSettlementNode`))
  ;[1 1 1] test that settlement owner is set to correct player
  (if (!= (`/Game/BluePrints/BP_settlementNode.player` (`local.selectedSettlementNode`)) _currentplayer_2)
    (`KismetSystemLibrary.PrintString` (`KismetStringLibrary.Concat_StrStr` "ERROR: a player placed a settlement but is not its owner. \nPlayer \"" (`KismetSystemLibrary.GetDisplayName` _currentplayer_2) "\" clicked settlement \"" (`KismetSystemLibrary.GetDisplayName` _selectedsettlementnode_4) "\" but the settlement player value is \"" (`KismetSystemLibrary.GetDisplayName` (`/Game/BluePrints/BP_settlementNode.player` _selectedsettlementnode_4)) "\".") true true (struct :`R` 1.0 :`A` 1.0) 10.0))
  ;[1 1 1] test that owned settlements are added to player "settlements" list
  (if (not (`KismetArrayLibrary.Array_Contains` (`/Game/BluePrints/BP_player.settlements` _currentplayer_3) _selectedsettlementnode))
    (`KismetSystemLibrary.PrintString` (`KismetStringLibrary.Concat_StrStr` "ERROR: settlement was not added to player owned settlement list. \nPlayer \"" (`KismetSystemLibrary.GetDisplayName` _currentplayer_3) "\" took ownership of settlement node \"" (`KismetSystemLibrary.GetDisplayName` _selectedsettlementnode) "\" but the settlement was not added to the player's owned settlement list.") true true (struct :`R` 1.0 :`A` 1.0) 10.0))
  ;[1 1 1] test if player colour and settlement colour match after claiming
  (if (`|EnumInequality` _colour_2 _colour)
    (`KismetSystemLibrary.PrintString` (`KismetStringLibrary.Concat_StrStr` "ERROR: after setting settlement as owned, settlement colour and player colour do not match. \nPlayer \"" (`KismetSystemLibrary.GetDisplayName` _currentplayer) "\" with colour \"" (`|GetEnumeratorNameAsString` _colour_2) "\" took ownership of \"" (`KismetSystemLibrary.GetDisplayName` _selectedsettlementnode_2) "\" but it has colour \"" (`|GetEnumeratorNameAsString` _colour) "\".") true true (struct :`R` 1.0 :`A` 1.0) 10.0))
  ;[1 1 1] test if game manager's settled nodes list contains the correct settlement nodes
  (bind _output_get_2 (set `local.iteratorNode` (`local.selectedSettlementNode`)))
  (if (`KismetArrayLibrary.Array_Contains` (`/Game/BluePrints/BP_gameManager.SettledNodes` (`self.gameManagerRef`)) _output_get_2)
    (for _array_element_2 (`/Game/BluePrints/BP_settlementNode.adjacentRoads` _selectedsettlementnode_3)
      (if (== (`/Game/BluePrints/BP_road.nodeA` _array_element_2) _selectedsettlementnode_3)
        (set `local.iteratorNode` (`/Game/BluePrints/BP_road.nodeB` _array_element_2))
        (else
          (set `local.iteratorNode` (`/Game/BluePrints/BP_road.nodeA` _array_element_2))))
      (if (not (`KismetArrayLibrary.Array_Contains` (`/Game/BluePrints/BP_gameManager.SettledNodes` (`self.gameManagerRef`)) (`local.iteratorNode`)))
        (`KismetSystemLibrary.PrintString` (`KismetStringLibrary.Concat_StrStr` "ERROR: settled node not in settled nodes list. \nPlayer \"" (`KismetSystemLibrary.GetDisplayName` (`/Game/BluePrints/BP_gameManager.currentPlayer` (`self.gameManagerRef`))) "\" claimed node \"" (`KismetSystemLibrary.GetDisplayName` (`local.selectedSettlementNode`)) "\" making the node \"" (`KismetSystemLibrary.GetDisplayName` (`local.iteratorNode`)) "\" unavailable but it is not in the game manager's SettledNodes list.") true true (struct :`R` 1.0 :`A` 1.0) 10.0 :!label _label)
        (break)))
    ;[1 1 1] test if settlements disappeared after one was placed
    (for _array_element_3 (`/Game/BluePrints/BP_gameManager.settlementsNodes` (`self.gameManagerRef`))
      (if (`KismetArrayLibrary.Array_Contains` (`/Game/BluePrints/BP_gameManager.SettledNodes` (`self.gameManagerRef`)) _array_element_3)
        _
        (elif (`SceneComponent.IsVisible` (`/Game/BluePrints/BP_settlementNode.Sphere` _array_element_3))
          (`KismetSystemLibrary.PrintString` (`KismetStringLibrary.Concat_StrStr` "ERROR: not settled spheres were visible after a settlement was placed. \nOne such node is \"" (`KismetSystemLibrary.GetDisplayName` _array_element_3) "\".") true true (struct :`R` 1.0 :`A` 1.0) 10.0)
          (break))))
    ;[1 1 1] test if settlement clicking disabled after settlement placed
    (if (or (`|EnumEquality` _clickstate_2 "NewEnumerator0") _benableclickevents_2)
      (`KismetSystemLibrary.PrintString` (`KismetStringLibrary.Concat_StrStr` "ERROR: settlements still placable after settlement placed. \nClick state is \"" (`|GetEnumeratorNameAsString` _clickstate_2) "\" and click events enabled is \"" (`KismetStringLibrary.Conv_BoolToString` _benableclickevents_2) "\".") true true (struct :`R` 1.0 :`A` 1.0) 10.0))
    (else
      (goto _label))))

(fn `unitTestMapObjects`
  (locals (allHexes :type "Set of /Game/BluePrints/BP_hexGrid Object Reference") (hexRefSet :type "Set of /Game/BluePrints/BP_hexGrid Object Reference") (quitOnCompletion :type Boolean) (firstRoadRefError :type Boolean) (firstNoneError :type Boolean :default true) (firstNoRefError :type Boolean :default true) (first6RefError :type Boolean :default true) (hexRefCount :type "Map of /Game/BluePrints/BP_hexGrid Object Reference to /Game/Data/UnitTests/S_settlementNodeSet Structure"))
  (bind _hexrefcount (`local.hexRefCount`))
  ;[1 1 1] road refs to settlement nodes are not None
  (bind _outactors (`GameplayStatics.GetAllActorsOfClass` "/Game/BluePrints/BP_road.BP_road_C"))
  (for _array_element _outactors
    (bind _returnvalue (not (`KismetSystemLibrary.IsValid` (`/Game/BluePrints/BP_road.nodeA` _array_element))))
    (if (or _returnvalue (not (`KismetSystemLibrary.IsValid` (`/Game/BluePrints/BP_road.nodeB` _array_element))))
      (`KismetSystemLibrary.PrintString` "ERROR: Road does not have a reference to 2 settlement nodes" true true (struct :`R` 1.0 :`A` 1.0) 10.0)
      (`KismetSystemLibrary.PrintString` (`KismetSystemLibrary.GetDisplayName` _array_element) true true (struct :`R` 1.0 :`A` 1.0) 10.0)
      (if _returnvalue
        (`KismetSystemLibrary.PrintString` "is missing Node A" true true (struct :`R` 1.0 :`A` 1.0) 10.0)
        (else
          (`KismetSystemLibrary.PrintString` "is missing Node B" true true (struct :`R` 1.0 :`A` 1.0) 10.0)))
      (set `local.quitOnCompletion` true)))
  (bind _outactors_2 (`GameplayStatics.GetAllActorsOfClass` "/Game/BluePrints/BP_settlementNode.BP_settlementNode_C"))
  (for _array_element_2 _outactors_2
    (bind _hexrefs (`/Game/BluePrints/BP_settlementNode.hexRefs` _array_element_2))
    ;[1 1 1] node refs to hexes are not None
    (for _array_element_3 _hexrefs
      (if (not (`KismetSystemLibrary.IsValid` _array_element_3))
        (if (`local.firstNoneError`)
          (`KismetSystemLibrary.PrintString` "ERROR: some settlements have hex references set to None" true true (struct :`R` 1.0 :`A` 1.0) 10.0)
          (set `local.firstNoneError` false)
          (`KismetSystemLibrary.PrintString` (`KismetSystemLibrary.GetDisplayName` _array_element_2) true true (struct :`R` 1.0 :`A` 1.0) 10.0)
          (break))))
    (bind _returnvalue_2 (`KismetArrayLibrary.Array_Length` _hexrefs))
    ;[1 1 1] settlement node has no hex reference
    (if (== _returnvalue_2 0)
      (`KismetSystemLibrary.PrintString` "ERROR: some settlement has no hex referenced" true true (struct :`R` 1.0 :`A` 1.0) 10.0)
      (`KismetSystemLibrary.PrintString` (`KismetSystemLibrary.GetDisplayName` _array_element_2) true true (struct :`R` 1.0 :`A` 1.0) 10.0)
      (set `local.quitOnCompletion` true)
      (else
        ;[1 1 1] settlement node has >3 hex references
        (if (> _returnvalue_2 3)
          (`KismetSystemLibrary.PrintString` "ERROR: some settlement references more than 3 hexes" true true (struct :`R` 1.0 :`A` 1.0) 10.0)
          (`KismetSystemLibrary.PrintString` (`KismetSystemLibrary.GetDisplayName` _array_element_2) true true (struct :`R` 1.0 :`A` 1.0) 10.0)
          (set `local.quitOnCompletion` true))))
    ;[1 1 1] create a set of all settlements that reference each hex to later ensure there are no duplicate references and that each hex is referenced 6 times
    (for _array_element_4 _hexrefs
      (if (`KismetSystemLibrary.IsValid` _array_element_4)
        (bind (_value _returnvalue_3) (`BlueprintMapLibrary.Map_Find` _hexrefcount _array_element_4))
        (if _returnvalue_3
          (if (`BlueprintSetLibrary.Set_Contains` (break `/Game/Data/UnitTests/S_settlementNodeSet` _value) _array_element_2)
            (`KismetSystemLibrary.PrintString` "ERROR: node references the same hex multiple times" true true (struct :`R` 1.0 :`A` 1.0) 10.0)
            (`KismetSystemLibrary.PrintString` (`KismetSystemLibrary.GetDisplayName` _array_element_2) true true (struct :`R` 1.0 :`A` 1.0) 10.0)
            (set `local.quitOnCompletion` true)
            (else
              (bind _set (`|MakeSet` _array_element_2))
              (bind _result (`BlueprintSetLibrary.Set_Union` (break `/Game/Data/UnitTests/S_settlementNodeSet` _value) _set))
              (`BlueprintMapLibrary.Map_Add` _hexrefcount _array_element_4 (make `/Game/Data/UnitTests/S_settlementNodeSet` _result))))
          (else
            (`BlueprintMapLibrary.Map_Add` _hexrefcount _array_element_4 (make `/Game/Data/UnitTests/S_settlementNodeSet` _set)))))))
  ;[1 1 1] check for any hexes that exist but are never referenced by a settlement node
  (`BlueprintSetLibrary.Set_Clear` (`local.allHexes`))
  (bind _outactors_3 (`GameplayStatics.GetAllActorsOfClass` "/Game/BluePrints/BP_hexGrid.BP_hexGrid_C"))
  (`BlueprintSetLibrary.Set_AddItems` (`local.allHexes`) _outactors_3)
  (bind _keys (`BlueprintMapLibrary.Map_Keys` (`local.hexRefCount`)))
  (`BlueprintSetLibrary.Set_AddItems` (`local.hexRefSet`) _keys)
  (bind _result_2 (`BlueprintSetLibrary.Set_Difference` (`local.allHexes`) (`local.hexRefSet`)))
  (if (!= (`BlueprintSetLibrary.Set_Length` _result_2) 0)
    (if (`local.firstNoRefError`)
      (`KismetSystemLibrary.PrintString` "ERROR: some Hex(es) are not referenced by any settlement node" true true (struct :`R` 1.0 :`A` 1.0) 10.0)
      (set `local.firstNoRefError` false))
    (bind _result_3 (`BlueprintSetLibrary.Set_ToArray` _result_2))
    (for _array_element_5 _result_3
      (`KismetSystemLibrary.PrintString` (`KismetSystemLibrary.GetDisplayName` _array_element_5) true true (struct :`R` 1.0 :`A` 1.0) 10.0)))
  ;[1 1 1] check all hexes are referenced by exactly 6 nodes
  (bind _keys_2 (`BlueprintMapLibrary.Map_Keys` (`local.hexRefCount`)))
  (for _array_element_6 _keys_2
    (if (!= (`BlueprintSetLibrary.Set_Length` (break `/Game/Data/UnitTests/S_settlementNodeSet` (`BlueprintMapLibrary.Map_Find` (`local.hexRefCount`) _array_element_6))) 6)
      (if (`local.first6RefError`)
        (`KismetSystemLibrary.PrintString` "ERROR: some Hex(es) are not referenced by exactly 6 nodes" true true (struct :`R` 1.0 :`A` 1.0) 10.0)
        (set `local.first6RefError` false))
      (`KismetSystemLibrary.PrintString` (`KismetSystemLibrary.GetDisplayName` _array_element_6) true true (struct :`R` 1.0 :`A` 1.0) 10.0)
      (set `local.quitOnCompletion` true)))
  (if (`local.quitOnCompletion`)
    (`KismetSystemLibrary.QuitGame` null "Quit")))

(fn `unitTestPlayer`
  (bind _outactors (`GameplayStatics.GetAllActorsOfClass` "/Game/BluePrints/BP_player.BP_player_C"))
  ;[1 1 1] at least one player object exists at start of game
  (if (< (`KismetArrayLibrary.Array_Length` _outactors) 4)
    (for _index (range 4)
      (if (not (`KismetSystemLibrary.IsValid` (`|GetArrayItem` _outactors _index)))
        (`KismetSystemLibrary.PrintString` "ERROR: less than 4 players were instantiated at the start of game" true true (struct :`R` 1.0 :`A` 1.0) 10.0)
        (break)))
    (bind _returnvalue (`GameplayStatics.GetActorOfClass` "/Game/BluePrints/BP_player.BP_player_C"))
    (bind _enumvalue (foreach `/Game/Data/E_resourceType` false)
      (:`LoopBody`
        ;[1 1 1] do not query player hand for desert cards
        (if (`|EnumInequality` _enumvalue "NewEnumerator6")
          (bind _hand_resourcecards (break `/Game/Data/S_Hand` (`/Game/BluePrints/BP_player.hand` _returnvalue)))
          (bind (_value _returnvalue_2) (`BlueprintMapLibrary.Map_Find` _hand_resourcecards _enumvalue))
          ;[1 1 1] hand keys should start instantiated
          (if _returnvalue_2
            ;[1 1 1] hand should start empty
            (if (!= _value 0)
              (`KismetSystemLibrary.PrintString` "ERROR: player hand should start empty" true true (struct :`R` 1.0 :`A` 1.0) 10.0)
              (`KismetSystemLibrary.PrintString` (`KismetStringLibrary.Concat_StrStr` (`KismetSystemLibrary.GetDisplayName` _returnvalue) ": has " (`KismetStringLibrary.Conv_IntToString` _value) " " (`|GetEnumeratorNameAsString` _enumvalue)) true true (struct :`R` 1.0 :`A` 1.0) 10.0))
            (else
              (`KismetSystemLibrary.PrintString` "ERROR: player hand struct is missing some resource keys from map  \nFATAL: cannot continue tests" true true (struct :`R` 1.0 :`A` 1.0) 10.0)
              (return)))))
      (:`then`
        ;[1 1 1] adding resources works
        (`/Game/BluePrints/BP_player.addResource` _returnvalue "NewEnumerator0" 1)
        (bind _hand_resourcecards_2 (break `/Game/Data/S_Hand` (`/Game/BluePrints/BP_player.hand` _returnvalue)))
        (if (== (`BlueprintMapLibrary.Map_Find` _hand_resourcecards_2 "NewEnumerator0") 1)
          ;[1 1 1] removing resources works
          (`/Game/BluePrints/BP_player.removeResource` _returnvalue "NewEnumerator0" 1)
          (bind _hand_resourcecards_3 (break `/Game/Data/S_Hand` (`/Game/BluePrints/BP_player.hand` _returnvalue)))
          (if (not (== (`BlueprintMapLibrary.Map_Find` _hand_resourcecards_3 "NewEnumerator0") 0))
            (`KismetSystemLibrary.PrintString` "ERROR: removing player resource did not work" true true (struct :`R` 1.0 :`A` 1.0) 10.0)
            (return))
          (else
            (`KismetSystemLibrary.PrintString` "ERROR: adding resource did not work" true true (struct :`R` 1.0 :`A` 1.0) 10.0)
            (`KismetSystemLibrary.PrintString` (`KismetStringLibrary.Concat_StrStr` "Player \"" (`KismetSystemLibrary.GetDisplayName` _returnvalue) "\" did not get resource") true true (struct :`R` 1.0 :`A` 1.0) 10.0)
            (return)))))))

(fn `unitTestRobber`
  (locals (robberRef :type "/Game/BluePrints/BP_robber Object Reference") (robberCoords :type "Vector Structure") (desertTile :type "/Game/BluePrints/BP_hexGrid Object Reference") (lastRobberHex :type "/Game/BluePrints/BP_hexGrid Object Reference") (currentPlayer :type "/Game/BluePrints/BP_player Object Reference") (selectedHex :type "/Game/BluePrints/BP_hexGrid Object Reference") (initialResourceQuantity :type Integer) (closestHexToRobber :type "/Game/BluePrints/BP_hexGrid Object Reference") (closestHexDistanceFromRobber :type "Float (double-precision)"))
  (bind _selectedhex (`local.selectedHex`))
  (bind _selectedhex_2 (`local.selectedHex`))
  (bind _closesthextorobber (`local.closestHexToRobber`))
  (bind _robberref (`local.robberRef`))
  (bind _currentlocation (`/Game/BluePrints/BP_robber.currentLocation` (`local.robberRef`)))
  (bind _resourcetype (`/Game/BluePrints/BP_hexGrid.resourceType` _selectedhex))
  (bind _currentlocation_2 (`/Game/BluePrints/BP_robber.currentLocation` _robberref))
  (bind _output (`|GetArrayItem` (`/Game/BluePrints/BP_hexGrid.settlementsNodes` _selectedhex)))
  (bind _player (`/Game/BluePrints/BP_settlementNode.player` _output))
  (bind _hand_resourcecards (break `/Game/Data/S_Hand` (`/Game/BluePrints/BP_player.hand` _player)))
  (bind _value (`BlueprintMapLibrary.Map_Find` _hand_resourcecards _resourcetype))
  ;[1 1 1] get variables
  (bind _returnvalue (`GameplayStatics.GetActorOfClass` "/Game/BluePrints/BP_robber.BP_robber_C"))
  (set `local.robberRef` _returnvalue)
  (set `local.lastRobberHex` (`/Game/BluePrints/BP_robber.currentLocation` (`local.robberRef`)))
  (bind _outactors (`GameplayStatics.GetAllActorsOfClass` "/Game/BluePrints/BP_hexGrid.BP_hexGrid_C"))
  (for _array_element _outactors
    (if (`|EnumEquality` (`/Game/BluePrints/BP_hexGrid.resourceType` _array_element) "NewEnumerator6")
      (set `local.desertTile` _array_element)
      (break)))
  ;[1 1 1] temp variable setup
  (set `local.currentPlayer` (`/Game/BluePrints/BP_gameManager.currentPlayer` (`self.gameManagerRef`)))
  ;[1 1 1] test if robber started on desert tile
  (if (!= (`local.lastRobberHex`) (`local.desertTile`))
    (`KismetSystemLibrary.PrintString` (`KismetStringLibrary.Concat_StrStr` "ERROR: Robber started on wrong tile \nRobber should have been on hex \"" (`KismetSystemLibrary.GetDisplayName` (`local.desertTile`)) "\" \nbut was actually on hex \"" (`KismetSystemLibrary.GetDisplayName` (`local.lastRobberHex`)) "\"") true true (struct :`R` 1.0 :`A` 1.0) 10.0))
  ;[1 1 1] test if robber moves when 7 rolled and different hex clicked
  (`/Game/BluePrints/BP_gameManager.Debug Roll Dice` (`self.gameManagerRef`) 7)
  (bind _outactors_2 (`GameplayStatics.GetAllActorsOfClass` "/Game/BluePrints/BP_hexGrid.BP_hexGrid_C"))
  (`KismetArrayLibrary.Array_RemoveItem` _outactors_2 (`local.lastRobberHex`))
  ;;[0.5 0.5 0.5] filter any hexes with no settlements (retain only hexes that give out resources)
  (for _array_element_2 _outactors_2
    (if (== (`KismetArrayLibrary.Array_Length` (`/Game/BluePrints/BP_hexGrid.settlementsNodes` _array_element_2)) 0)
      (`KismetArrayLibrary.Array_RemoveItem` _outactors_2 _array_element_2)))
  (bind _output_get (set `local.selectedHex` (`KismetArrayLibrary.Array_Random` _outactors_2)))
  (`/Game/BluePrints/BP_hexGrid.Debug Clicked(robberCube)` _output_get) ; click random hex tile to move robber
  (if (!= _currentlocation _output_get)
    (`KismetSystemLibrary.PrintString` (`KismetStringLibrary.Concat_StrStr` "ERROR: robber did not move to new hex when hex clicked. \nOn the turn of player \"" (`KismetSystemLibrary.GetDisplayName` (`local.currentPlayer`)) "\" a 7 was rolled and hex \"" (`KismetSystemLibrary.GetDisplayName` _output_get) "\" was clicked \nthe robber was on hex \"" (`KismetSystemLibrary.GetDisplayName` (`local.lastRobberHex`)) "\" and moved to hex \"" (`KismetSystemLibrary.GetDisplayName` _currentlocation) "\"") true true (struct :`R` 1.0 :`A` 1.0) 10.0))
  ;[1 1 1] Comment
  (set `local.robberCoords` (`self.K2_GetActorLocation` (`local.robberRef`)))
  (bind _outactors_3 (`GameplayStatics.GetAllActorsOfClass` "/Game/BluePrints/BP_hexGrid.BP_hexGrid_C"))
  (set `local.closestHexToRobber` (`|GetArrayItem` _outactors_3))
  (for _array_element_3 _outactors_3
    (bind _returnvalue_2 (`KismetMathLibrary.Vector_Distance` (`self.K2_GetActorLocation` _array_element_3) (`local.robberCoords`)))
    (if (< _returnvalue_2 (`local.closestHexDistanceFromRobber`))
      (set `local.closestHexToRobber` _array_element_3)
      (set `local.closestHexDistanceFromRobber` _returnvalue_2)))
  (if (!= _closesthextorobber _currentlocation_2)
    (`KismetSystemLibrary.PrintString` (`KismetStringLibrary.Concat_StrStr` "ERROR: Robber currentLocation does not match the hex closest to robber. \nRobber current location is \"" (`KismetSystemLibrary.GetDisplayName` _currentlocation_2) "\" with coordinates \"" (`KismetStringLibrary.Conv_VectorToString` (`self.K2_GetActorLocation` _currentlocation_2)) "\". \nClosest hex to robber is \"" (`KismetSystemLibrary.GetDisplayName` _closesthextorobber) "\" with coordinates \"" (`KismetStringLibrary.Conv_VectorToString` (`self.K2_GetActorLocation` _closesthextorobber)) "\". \nRobber coordinates are \"" (`KismetStringLibrary.Conv_VectorToString` (`self.K2_GetActorLocation` _robberref)) "\".") true true (struct :`R` 1.0 :`A` 1.0) 10.0))
  ;[1 1 1] test for robber's hex not giving out resources
  (bind _output_get_2 (set `local.selectedHex` (`/Game/BluePrints/BP_robber.currentLocation` (`local.robberRef`))))
  (if (> (`KismetArrayLibrary.Array_Length` (`/Game/BluePrints/BP_hexGrid.settlementsNodes` _output_get_2)) 0)
    (bind _output_get_3 (set `local.initialResourceQuantity` _value))
    (`/Game/BluePrints/BP_gameManager.Debug Roll Dice` (`self.gameManagerRef`) (`/Game/BluePrints/BP_hexGrid.tileNumber` (`local.selectedHex`)))
    (if (!= _output_get_3 _value)
      (`KismetSystemLibrary.PrintString` (`KismetStringLibrary.Concat_StrStr` "ERROR: Player gained resources when they should not have. \nA dice result of \"" (`KismetStringLibrary.Conv_IntToString` (`/Game/BluePrints/BP_die.lastRoll` (`/Game/BluePrints/BP_gameManager.dice1` (`self.gameManagerRef`)))) "\" was rolled and hex \"" (`KismetSystemLibrary.GetDisplayName` _selectedhex_2) "\" has number \"" (`KismetStringLibrary.Conv_IntToString` (`/Game/BluePrints/BP_hexGrid.tileNumber` _selectedhex_2)) "\". \nPlayer \"" (`KismetSystemLibrary.GetDisplayName` _player) "\" has a settlement adjacent to that hex. \nBefore the roll that player had \"" (`KismetStringLibrary.Conv_IntToString` (`local.initialResourceQuantity`)) "\" \"" (`|GetEnumeratorNameAsString` _resourcetype) "\" and now they have \"" (`KismetStringLibrary.Conv_IntToString` _value) "\". \nTheir adjacent settlement is \"" (`KismetSystemLibrary.GetDisplayName` _output) "\". \nThe  robber was on that hex and should have blocked resource gain.") true true (struct :`R` 1.0 :`A` 1.0) 10.0))
    (else
      (`KismetSystemLibrary.PrintString` (`KismetStringLibrary.Concat_StrStr` "ERROR: Cannot test robber resource blocking. \nRobber should have been on a hex with at least 1 settlement. \nInstead, robber is on hex \"" (`KismetSystemLibrary.GetDisplayName` _output_get_2) "\".") true true (struct :`R` 1.0 :`A` 1.0) 10.0))))

(fn `UserConstructionScript`)