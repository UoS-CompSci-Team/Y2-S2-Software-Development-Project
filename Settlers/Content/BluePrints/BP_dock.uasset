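; BP_dock is a trade dock actor for a resource-trading game, set up for one resource type or as a general dock.
; Its initialiseDock event puts the matching icon texture on the W_dockResource widget held by its widget component and turns off that component's shadow.
; It also sets TradeRatio, giving general docks a higher ratio than resource-specific ones.
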(event `initialise Dock`
  (params (resource :type "/Game/Data/E_dockType Enum" :default "NewEnumerator0"))
  (bind _asw_dock_resource (cast `/Game/UserInterface/W_dockResource` (`WidgetComponent.GetWidget` (`self.Widget`))))
  (switch `/Game/Data/E_dockType` resource
    (:`NewEnumerator1`
      (bind _resource (`/Game/UserInterface/W_dockResource.resource` _asw_dock_resource))
      (`Border.SetBrushFromTexture` _resource "/Game/UIAssets/dock/general.general")
      (set `self.tradeRatio` 3))
    (:`NewEnumerator2`
      (`Border.SetBrushFromTexture` _resource "/Game/UIAssets/dock/lumber.lumber")
      (set `self.tradeRatio` 2 :!label _label))
    (:`NewEnumerator3`
      (`Border.SetBrushFromTexture` _resource "/Game/UIAssets/dock/wool.wool")
      (goto _label))
    (:`NewEnumerator4`
      (`Border.SetBrushFromTexture` _resource "/Game/UIAssets/dock/brick.brick")
      (goto _label))
    (:`NewEnumerator5`
      (`Border.SetBrushFromTexture` _resource "/Game/UIAssets/dock/ore.ore")
      (goto _label))
    (:`NewEnumerator6`
      (`Border.SetBrushFromTexture` _resource "/Game/UIAssets/dock/corn.corn")
      (goto _label)))
  (`PrimitiveComponent.SetCastShadow` (`self.Widget`) false))

(fn `UserConstructionScript`)