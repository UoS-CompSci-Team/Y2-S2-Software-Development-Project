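; BP_bank is the game's bank, holding resource and special (development) cards in a BankHand struct.
; Functions check, add and remove resources by looping over map keys, with edits made on a temporary map and written back to the hand.
; PayPlayer branches on GameManager.HandHasAtLeast to either log a shortage or transfer resources and log gains.
; GiveDevCard moves a random special card to the current player through GameManager.
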(fn `addResourcesToBank`
  (params (resourcesToAdd :type "Map of /Game/Data/E_resourceType Enum to Integer"))
  (locals (tempResourceCardMap :type "Map of /Game/Data/E_resourceType Enum to Object Object Reference"))
  (bind (_bankhand_resourcecards _bankhand_specialcards) (break `/Game/Data/S_Hand` (`self.BankHand`)))
  (bind _tempresourcecardmap (`local.tempResourceCardMap`))
  ;[1 1 1] Get all keys of resources to add, duplicate hand into new temporary map, output keys as array
  (set `local.tempResourceCardMap` _bankhand_resourcecards)
  (bind _keys (`BlueprintMapLibrary.Map_Keys` resourcesToAdd))
  (for _array_element _keys
    (`BlueprintMapLibrary.Map_Add` _tempresourcecardmap _array_element (+ (`BlueprintMapLibrary.Map_Find` _tempresourcecardmap _array_element) (`BlueprintMapLibrary.Map_Find` resourcesToAdd _array_element))))
  ;[1 0 0] After loop is completed, set Bank hand to be duplicate hand (May be an issue)
  (`|VariableSetRef` (`self.BankHand`) (make `/Game/Data/S_Hand` (`local.tempResourceCardMap`) _bankhand_specialcards)))

(fn `checkBankResources`
  (params (resourcesToCheck :type "Map of /Game/Data/E_resourceType Enum to Integer"))
  (returns (`checkSucceded?` :type Boolean))
  (bind _bankhand_resourcecards (break `/Game/Data/S_Hand` (`self.BankHand`)))
  ;[1 1 1] for each key value do...
  (bind _keys (`BlueprintMapLibrary.Map_Keys` resourcesToCheck))
  (for _array_element _keys
    ;[1 1 1] if bank does not have resource, return false and break
    (if (not (>= (`BlueprintMapLibrary.Map_Find` _bankhand_resourcecards _array_element) (`BlueprintMapLibrary.Map_Find` resourcesToCheck _array_element)))
      (return false)))
  (return true) ; If all checks have passed correctly, return true
)

(fn `checkRemainingDevCards`
  (returns (devCardsRemaining :type Boolean))
  (bind (_bankhand_resourcecards _bankhand_specialcards) (break `/Game/Data/S_Hand` (`self.BankHand`)))
  (if (<= (`BlueprintMapLibrary.Map_Length` _bankhand_specialcards) 0)
    (return false)
    (else
      (return true))))

(fn `giveDevCard`
  (returns (SpecialCard :type "/Game/Data/E_specialType Enum"))
  (bind (_bankhand_resourcecards _bankhand_specialcards) (break `/Game/Data/S_Hand` (`self.bankHand`)))
  (bind _gamemanager (`self.gameManager`))
  (bind (_hand_resourcecards _hand_specialcards) (break `/Game/Data/S_Hand` (`/Game/BluePrints/BP_player.hand` (`/Game/BluePrints/BP_gameManager.currentPlayer` _gamemanager))))
  ;[0.135 0 1] Sprint 5
  (bind (_resourcecard _specialcard) (`/Game/BluePrints/BP_gameManager.pickRandomCard` _gamemanager (`self.bankHand`) false))
  (`BlueprintMapLibrary.Map_Add` _hand_specialcards _specialcard (+ (`BlueprintMapLibrary.Map_Find` _hand_specialcards _specialcard) 1))
  (`BlueprintMapLibrary.Map_Add` _bankhand_specialcards _specialcard (- (`BlueprintMapLibrary.Map_Find` _bankhand_specialcards _specialcard) 1))
  (return _specialcard))

(fn `payPlayer`
  (params (playerToPay :type "/Game/BluePrints/BP_player Object Reference") (resourcesToPay :type "Map of /Game/Data/E_resourceType Enum to Integer"))
  (bind _resourcestopay (`local.resourcesToPay`))
  ;[1 1 1] check quantities
  (bind _transactioninvalid (`/Game/BluePrints/BP_gameManager.handHasAtLeast` (`self.gameManager`) (`self.bankHand`) (make `/Game/Data/S_Hand` resourcesToPay)))
  (if _transactioninvalid
    ;[1 1 1] failed log output
    (`/Game/UserInterface/W_MainUI.addToGameLog` (`/Game/BluePrints/BP_gameManager.mainUI` (`self.gameManager`)) (`KismetStringLibrary.Concat_StrStr` "Bank tried to pay " (`/Game/BluePrints/BP_player.loggablePlayerName` playerToPay) " but did not have the resources!"))
    (else
      (`self.removeResourcesFromBank` resourcesToPay)
      (`/Game/BluePrints/BP_player.addResourcesAlpha` playerToPay resourcesToPay)
      ;[1 1 1] Add to game log
      (bind _keys (`BlueprintMapLibrary.Map_Keys` _resourcestopay))
      (for _array_element _keys
        (bind _value (`BlueprintMapLibrary.Map_Find` _resourcestopay _array_element))
        (if (!= _value 0)
          (`/Game/UserInterface/W_MainUI.addToGameLog` (`/Game/BluePrints/BP_gameManager.mainUI` (`self.gameManager`)) (`KismetStringLibrary.Concat_StrStr` (`/Game/BluePrints/BP_player.loggablePlayerName` (`local.playerToPay`)) " gained " (`KismetStringLibrary.Conv_IntToString` _value) " " (`|GetEnumeratorNameAsString` _array_element) "!")))))))

(fn `removeResourcesFromBank`
  (params (`Resources To Remove` :type "Map of /Game/Data/E_resourceType Enum to Integer"))
  (locals (tempResourceCardMap :type "Map of /Game/Data/E_resourceType Enum to Object Object Reference"))
  (bind (_bankhand_resourcecards _bankhand_specialcards) (break `/Game/Data/S_Hand` (`self.BankHand`)))
  (bind _tempresourcecardmap (`local.tempResourceCardMap`))
  ;[1 1 1] Get all keys of resources to subtract, duplicate hand into new temporary map, output keys as array
  (set `local.tempResourceCardMap` _bankhand_resourcecards)
  (bind _keys (`BlueprintMapLibrary.Map_Keys` `Resources To Remove`))
  (for _array_element _keys
    (`BlueprintMapLibrary.Map_Add` _tempresourcecardmap _array_element (- (`BlueprintMapLibrary.Map_Find` _tempresourcecardmap _array_element) (`BlueprintMapLibrary.Map_Find` `Resources To Remove` _array_element))))
  ;[1 0 0] After loop is completed, set bank hand to be duplicate hand (May be an issue)
  (`|VariableSetRef` (`self.BankHand`) (make `/Game/Data/S_Hand` (`local.tempResourceCardMap`) _bankhand_specialcards)))

(fn `UserConstructionScript`)