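; Robber piece for a hex-board resource game, which starts on the desert hex and tracks the hex it occupies.
; On BeginPlay it caches BP_gameManager and finds the desert BP_hexGrid by resource type.
; Moves run through a timeline, but MoveRobber ignores its alpha and snaps to an offset from the hex.
; PlayerPlaceRobber shows RobberHex markers on every other hex and enables click events.
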(event `self.ReceiveBeginPlay`
  (bind _returnvalue (`GameplayStatics.GetActorOfClass` "/Game/BluePrints/BP_gameManager.BP_gameManager_C"))
  (set `self.gameManager` _returnvalue)
  (`self.setToDesert`))

(event `moveRobberEvent`
  (params (hex :type "/Game/BluePrints/BP_hexGrid Object Reference"))
  (bind (_direction _newtrack_0) (`Timeline|Timeline_0`)
    (:`Update`
      (`self.moveRobber` hex _newtrack_0))))

(fn `getLocation`
  (returns (hex :type "/Game/BluePrints/BP_hexGrid Object Reference"))
  (return (`self.currentLocation`)))

(fn `moveRobber`
  (params (hex :type "/Game/BluePrints/BP_hexGrid Object Reference") (alpha :type "Float (double-precision)"))
  ;[1 1 1] Moves robber to a hex and updates current location hex
  (`self.K2_SetActorLocation` (+ (`self.K2_GetActorLocation` hex) (30.0 30.0 0.0)))
  (`self.setLocation` hex))

(fn `playerPlaceRobber`
  (locals (availableRobberHexes :type "Array of /Game/BluePrints/BP_hexGrid Object Reference"))
  ;[1 1 1] set an array of hexes without current robber location
  (for _array_element (`/Game/BluePrints/BP_gameManager.hex's` (`self.gameManager`))
    (if (not (== _array_element (`self.currentLocation`)))
      (`SceneComponent.SetVisibility` (`/Game/BluePrints/BP_hexGrid.robberHex` _array_element) true false)
      (set `PlayerController.bEnableClickEvents` true (`GameplayStatics.GetPlayerController` 0)))))

(fn `setLocation`
  (params (hex :type "/Game/BluePrints/BP_hexGrid Object Reference"))
  (set `self.currentLocation` hex))

(fn `setToDesert`
  (`KismetSystemLibrary.PrintString` "robber to desert fired")
  (bind _outactors (`GameplayStatics.GetAllActorsOfClass` "/Game/BluePrints/BP_hexGrid.BP_hexGrid_C"))
  (for _array_element _outactors
    (if (`|EnumEquality` (`/Game/BluePrints/BP_hexGrid.resourceType` _array_element) "NewEnumerator6")
      (`self.moveRobberEvent` _array_element)
      (break))))

(fn `UserConstructionScript`)