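; Bank trade object for a settlement-building resource game, exchanging the current player's resource cards with the bank.
; The construction script builds per-resource trade rates from docks beside the player's settlements, with general docks lowering rates above three.
; Add/remove functions edit sending and receiving maps, with checks against player and bank hands.
; Validation requires sent cards to divide evenly by rate and match the requested total, while MoveItems pays both sides.
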(event `self.addItemToReceiving`
  (params (resourceCard :type "/Game/Data/E_resourceType Enum" :default "NewEnumerator7"))
  (`self.addItemToReceiving_` resourceCard))

(event `self.addItemToSending`
  (params (resourceCard :type "/Game/Data/E_resourceType Enum" :default "NewEnumerator7"))
  (`self.addItemToSending_` resourceCard))

(event `self.removeItemFromSending`
  (params (resourceCard :type "/Game/Data/E_resourceType Enum" :default "NewEnumerator7"))
  (`self.removeItemFromSending_` resourceCard))

(event `self.removeItemFromReceiving`
  (params (resourceCard :type "/Game/Data/E_resourceType Enum" :default "NewEnumerator7"))
  (`self.removeItemFromReceiving_` resourceCard))

(event `self.moveItems`
  (`self.moveItems_`))

(fn `addItemToReceiving_`
  (params (resourceCard :type "/Game/Data/E_resourceType Enum" :default "NewEnumerator7"))
  (bind _receivingitems (`self.receivingItems`))
  (`BlueprintMapLibrary.Map_Add` _receivingitems resourceCard (+ (`BlueprintMapLibrary.Map_Find` _receivingitems resourceCard) 1)))

(fn `addItemToSending_`
  (params (resourceCard :type "/Game/Data/E_resourceType Enum" :default "NewEnumerator7"))
  (bind _sendingitems (`self.sendingItems`))
  (`BlueprintMapLibrary.Map_Add` _sendingitems resourceCard (+ (`BlueprintMapLibrary.Map_Find` _sendingitems resourceCard) 1)))

(fn `canReceiverIncreaseResource`
  (params (resourceCard :type "/Game/Data/E_resourceType Enum" :default "NewEnumerator7"))
  (returns (canIncrease :type Boolean))
  (bind _canincrease (`self.canReceiverIncreaseResource_` resourceCard))
  (return _canincrease))

(fn `canReceiverIncreaseResource_`
  (params (resourceCard :type "/Game/Data/E_resourceType Enum" :default "NewEnumerator7"))
  (returns (canIncrease :type Boolean))
  (return (< (`BlueprintMapLibrary.Map_Find` (`self.receivingItems`) resourceCard) (`BlueprintMapLibrary.Map_Find` (`.resourceCards_6_629E6944473B44BFE5C01789E3CC3565` (break `/Game/Data/S_Hand` (`/Game/BluePrints/BP_bank.bankHand` (`/Game/BluePrints/BP_gameManager.bank` (`self.gameManager`))))) resourceCard))))

(fn `canSenderIncreaseResource`
  (params (resourceCard :type "/Game/Data/E_resourceType Enum" :default "NewEnumerator7"))
  (returns (canIncrease :type Boolean))
  (bind _canincrease (`self.canSenderIncreaseResource_` resourceCard))
  (return _canincrease))

(fn `canSenderIncreaseResource_`
  (params (resourceCard :type "/Game/Data/E_resourceType Enum" :default "NewEnumerator7"))
  (returns (canIncrease :type Boolean))
  (return (< (`BlueprintMapLibrary.Map_Find` (`self.sendingItems`) resourceCard) (`BlueprintMapLibrary.Map_Find` (`.resourceCards_6_629E6944473B44BFE5C01789E3CC3565` (break `/Game/Data/S_Hand` (`/Game/BluePrints/BP_player.hand` (`self.sender`)))) resourceCard))))

(fn `getSender`
  (returns (sender :type "/Game/BluePrints/BP_player Object Reference"))
  (return (`self.sender`)))

(fn `isTradeValid`
  (returns (valid :type Boolean))
  (locals (divisionSum :type Integer) (remainderSum :type Integer) (receivingItemsSum :type Integer))
  (bind _sendingitems (`self.sendingItems`))
  (bind _traderate (`self.tradeRate`))
  (if (or (`BlueprintMapLibrary.Map_IsEmpty` (`self.receivingItems`)) (`BlueprintMapLibrary.Map_IsEmpty` (`self.sendingItems`)))
    (return false)
    (else
      (bind _keys (`BlueprintMapLibrary.Map_Keys` _sendingitems))
      (bind _values (`BlueprintMapLibrary.Map_Values` _sendingitems))
      (for _index (range (`KismetArrayLibrary.Array_Length` _values))
        (switch `/Game/Data/E_resourceType` (`|GetArrayItem` _keys _index)
          (:`NewEnumerator0`
            (bind _output (`|GetArrayItem` _values _index))
            (bind (_remainder _returnvalue) (`KismetMathLibrary.FMod` (`KismetMathLibrary.Conv_IntToDouble` _output) (`KismetMathLibrary.Conv_IntToDouble` (`BlueprintMapLibrary.Map_Find` _traderate "NewEnumerator4"))))
            (set `local.remainderSum` (`KismetMathLibrary.FTrunc` (+ (`local.remainderSum`) _remainder)))
            (set `local.divisionSum` (+ (`local.divisionSum`) _returnvalue)))
          (:`NewEnumerator1`
            (bind (_remainder_2 _returnvalue_2) (`KismetMathLibrary.FMod` (`KismetMathLibrary.Conv_IntToDouble` _output) (`KismetMathLibrary.Conv_IntToDouble` (`BlueprintMapLibrary.Map_Find` _traderate "NewEnumerator6"))))
            (set `local.remainderSum` (`KismetMathLibrary.FTrunc` (+ (`local.remainderSum`) _remainder_2)))
            (set `local.divisionSum` (+ (`local.divisionSum`) _returnvalue_2)))
          (:`NewEnumerator2`
            (bind (_remainder_3 _returnvalue_3) (`KismetMathLibrary.FMod` (`KismetMathLibrary.Conv_IntToDouble` _output) (`KismetMathLibrary.Conv_IntToDouble` (`BlueprintMapLibrary.Map_Find` _traderate "NewEnumerator3"))))
            (set `local.remainderSum` (`KismetMathLibrary.FTrunc` (+ (`local.remainderSum`) _remainder_3)))
            (set `local.divisionSum` (+ (`local.divisionSum`) _returnvalue_3)))
          (:`NewEnumerator4`
            (bind (_remainder_4 _returnvalue_4) (`KismetMathLibrary.FMod` (`KismetMathLibrary.Conv_IntToDouble` _output) (`KismetMathLibrary.Conv_IntToDouble` (`BlueprintMapLibrary.Map_Find` _traderate "NewEnumerator2"))))
            (set `local.remainderSum` (`KismetMathLibrary.FTrunc` (+ (`local.remainderSum`) _remainder_4)))
            (set `local.divisionSum` (+ (`local.divisionSum`) _returnvalue_4)))
          (:`NewEnumerator5`
            (bind (_remainder_5 _returnvalue_5) (`KismetMathLibrary.FMod` (`KismetMathLibrary.Conv_IntToDouble` _output) (`KismetMathLibrary.Conv_IntToDouble` (`BlueprintMapLibrary.Map_Find` _traderate "NewEnumerator5"))))
            (set `local.remainderSum` (`KismetMathLibrary.FTrunc` (+ (`local.remainderSum`) _remainder_5)))
            (set `local.divisionSum` (+ (`local.divisionSum`) _returnvalue_5)))))
      (if (== (`local.remainderSum`) 0)
        (bind _values_2 (`BlueprintMapLibrary.Map_Values` (`self.receivingItems`)))
        (for _array_element _values_2
          (set `local.receivingItemsSum` (+ _array_element (`local.receivingItemsSum`))))
        (if (== (`local.divisionSum`) (`local.receivingItemsSum`))
          (return true)
          (else
            (return false)))
        (else
          (return false))))))

(fn `isTradeValid_`
  (returns (Valid :type Boolean))
  (bind _valid (`self.isTradeValid`))
  (return _valid))

(fn `moveItems_`
  (`/Game/BluePrints/BP_player.payBank` (`self.sender`) (`self.sendingItems`))
  (`/Game/BluePrints/BP_bank.payPlayer` (`/Game/BluePrints/BP_gameManager.bank` (`self.gameManager`)) (`self.sender`) (`self.receivingItems`)))

(fn `removeItemFromReceiving_`
  (params (resourceCard :type "/Game/Data/E_resourceType Enum" :default "NewEnumerator7"))
  (bind _receivingitems (`self.receivingItems`))
  (bind _value (`BlueprintMapLibrary.Map_Find` _receivingitems resourceCard))
  (if (not (== _value 0))
    (`BlueprintMapLibrary.Map_Add` _receivingitems resourceCard (- _value 1))))

(fn `removeItemFromSending_`
  (params (resourceCard :type "/Game/Data/E_resourceType Enum" :default "NewEnumerator7"))
  (bind _sendingitems (`self.sendingItems`))
  (bind _value (`BlueprintMapLibrary.Map_Find` _sendingitems resourceCard))
  (if (not (== _value 0))
    (`BlueprintMapLibrary.Map_Add` _sendingitems resourceCard (- _value 1))))

(fn `UserConstructionScript`
  (bind _traderate (`self.tradeRate`))
  (bind _returnvalue (`GameplayStatics.GetActorOfClass` "/Game/BluePrints/BP_gameManager.BP_gameManager_C"))
  (bind _output_get (set `self.gameManager` _returnvalue))
  (bind _output_get_2 (set `self.sender` (`/Game/BluePrints/BP_gameManager.currentPlayer` _output_get)))
  ;[1 1 1] Iterates through each of the players docks
  (for _array_element (`/Game/BluePrints/BP_player.settlements` _output_get_2)
    (for _array_element_2 (`/Game/BluePrints/BP_settlementNode.adjacentDocks` _array_element)
      (bind _resourcetype (`/Game/BluePrints/BP_dock.resourceType` _array_element_2))
      ;[1 1 1] If equal to 'general' dock type
      (if (`|EnumEquality` _resourcetype "NewEnumerator1")
        ;[1 1 1] If player owns a general dock - iterate through tradeRate keys - setting each rate to 3 only if current rate is set to 4
        (bind _keys (`BlueprintMapLibrary.Map_Keys` _traderate))
        (for _array_element_3 _keys
          (if (> (`BlueprintMapLibrary.Map_Find` _traderate _array_element_3) 3)
            (`BlueprintMapLibrary.Map_Add` _traderate _array_element_3 3)))
        (else
          ;[1 1 1] Update tradeRate map with resource type and rate
          (`BlueprintMapLibrary.Map_Add` (`self.tradeRate`) _resourcetype (`/Game/BluePrints/BP_dock.tradeRatio` _array_element_2)))))))