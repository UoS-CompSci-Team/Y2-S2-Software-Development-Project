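; BP_hexGrid is a board hex tile that holds a resource type, a number and a list of settlement nodes.
; Its setter events apply a material per resource, hide the number on Desert and update the number text.
; It binds to BP_gameManager state updates, showing RobberCube during PlacingRobber unless the robber is already there.
; Clicking that cube sets the state to AwaitingChange and moves the robber to this hex if elsewhere.
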(event `self.ReceiveBeginPlay`
  ;[1 1 1] initialize
  (bind _returnvalue (`GameplayStatics.GetActorOfClass` "/Game/BluePrints/BP_gameManager.BP_gameManager_C"))
  (bind _output_get (set `self.gameManagerRef` _returnvalue))
  (add `/Game/BluePrints/BP_gameManager.gameStateUpdate` _output_get (delegate `gameStateUpdate`)))

(event `gameStateUpdate`
  ;[1 1 1] initialize
  (`self.gameStateUpdate_Process`))

(event `setResource`
  (bind _hex (`self.Hex`))
  (switch `/Game/Data/E_resourceType` (`self.resourceType`)
    (:`NewEnumerator0`
      (`PrimitiveComponent.SetMaterial` _hex 0 "/Game/StarterContent/Materials/M_Brick_Clay_Beveled.M_Brick_Clay_Beveled"))
    (:`NewEnumerator1`
      (`PrimitiveComponent.SetMaterial` _hex 0 "/Game/StarterContent/Props/Materials/M_Bush.M_Bush"))
    (:`NewEnumerator2`
      (`PrimitiveComponent.SetMaterial` _hex 0 "/Game/StarterContent/Materials/M_Concrete_Poured.M_Concrete_Poured"))
    (:`NewEnumerator4`
      (`PrimitiveComponent.SetMaterial` _hex 0 "/Game/StarterContent/Materials/M_Wood_Floor_Walnut_Polished.M_Wood_Floor_Walnut_Polished"))
    (:`NewEnumerator5`
      (`PrimitiveComponent.SetMaterial` _hex 0 "/Game/StarterContent/Props/Materials/M_Rock.M_Rock"))
    (:`NewEnumerator6`
      (`PrimitiveComponent.SetMaterial` _hex 0 "/Game/StarterContent/Materials/M_Rock_Sandstone.M_Rock_Sandstone")
      (`SceneComponent.SetVisibility` (`self.Num`) false false))))

(event `setNumber`
  (params (setNum :type Integer))
  (bind _output_get (set `self.tileNumber` setNum))
  (`TextRenderComponent.K2_SetText` (`self.Num`) (`KismetTextLibrary.Conv_IntToText` _output_get)))

(event `self.robberCube.OnClicked`
  (params (TouchedComponent :type "PrimitiveComponent Object Reference") (ButtonPressed :type "Key Structure"))
  (`self.hexClickFunction` :!label _label))

(event `Debug Clicked(robberCube)`
  (goto _label))

(event `gameStateUpdate_Process`
  ;[1 1 1] update visibility on game state change
  (`self.updateRobberCubeVisibility`))

(fn `addSettlement`
  (params (settlement :type "/Game/BluePrints/BP_settlementNode Object Reference"))
  (`KismetArrayLibrary.Array_Add` (`self.settlementsNodes`) settlement))

(fn `hexClickFunction`
  (bind _returnvalue (`GameplayStatics.GetActorOfClass` "/Game/BluePrints/BP_robber.BP_robber_C"))
  (bind _gamemanager (`/Game/BluePrints/BP_robber.gameManager` _returnvalue))
  (switch `/Game/Data/E_gameState` (`/Game/BluePrints/BP_gameManager.gameState` _gamemanager)
    (:`NewEnumerator20`
      (if (not (== (`/Game/BluePrints/BP_robber.currentLocation` _returnvalue) self))
        (`/Game/BluePrints/BP_gameManager.Change Game State` _gamemanager "NewEnumerator28")
        (`/Game/BluePrints/BP_robber.moveRobberEvent` (`/Game/BluePrints/BP_gameManager.robber` _gamemanager) self false)))))

(fn `updateRobberCubeVisibility`
  (`SceneComponent.SetVisibility` (`self.robberCube`) (and (`|EnumEquality` (`/Game/BluePrints/BP_gameManager.gameState` (`self.gameManagerRef`)) "NewEnumerator20") (!= (`/Game/BluePrints/BP_robber.currentLocation` (`/Game/BluePrints/BP_gameManager.robber` (`self.gameManagerRef`))) self)) false))

(fn `UserConstructionScript`)