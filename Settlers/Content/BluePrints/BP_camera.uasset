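; BP_camera is a camera actor that serves as the player's view, with mouse-wheel zoom.
; On BeginPlay it enables input, takes over player 0's view target, moves to a default transform, hides its helper cube and prints a controls hint.
; The wheel axis changes the spring arm length within clamped limits, and middle mouse restores the default length, which is applied without clamping.
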(event `self.ReceiveBeginPlay`
  (bind _returnvalue (`GameplayStatics.GetPlayerController` 0))
  ;[1 1 1] begin play, enables inputs and sets default camera view
  (`self.EnableInput` _returnvalue)
  (`PlayerController.SetViewTargetWithBlend` _returnvalue self 0.0 "VTBlend_Linear" 0.0 false)
  ;[1 1 1] sets location of camera
  (`self.K2_SetActorTransform` (`self.defaultCameraPos`))
  ;[1 1 1] hides cube in BP_camera
  (`SceneComponent.SetVisibility` (`self.Cube`) false false)
  ;[1 1 1] dev instructions print (can delete if not wanted)
  (`KismetSystemLibrary.PrintString` "mouse wheel to scroll, middle mouse button to reset view" true true (struct :`R` 0.71875 :`G` 0.429513 :`B` 0.050099 :`A` 1.0) 3.0))

(event `InputAxisKey|MouseWheelAxis`
  (params (AxisValue :type "Float (single-precision)"))
  ;[1 1 1] mouse wheel makes camera zoom
  (`self.cameraZoom` AxisValue))

(event `Key|MiddleMouseButton`
  (params (Key :type "Key Structure"))
  ;[1 1 1] middle mouse button resets spring arm back to default pos
  (:`Pressed`
    (`self.resetSpringArm`)))

(fn `cameraZoom`
  (params (axis :type "Float (double-precision)"))
  ;[1 1 1] Camera Zooms in and out
  (set `SpringArmComponent.TargetArmLength` (`KismetMathLibrary.FClamp` (+ (* axis -80.0) (`SpringArmComponent.TargetArmLength` (`self.SpringArm`))) 5.0 1000.0) (`self.SpringArm`)))

(fn `resetSpringArm`
  ;[1 1 1] sets spring arm back to default length (5000)
  (set `SpringArmComponent.TargetArmLength` (`self.defaultSpringArmLength`) (`self.SpringArm`)))

(fn `UserConstructionScript`)