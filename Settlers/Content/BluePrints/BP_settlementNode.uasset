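; BP_settlementNode is a clickable board spot where a player can build a settlement.
; On BeginPlay it caches BP_gameManager; a sphere click or a debug event runs the settlement click logic.
; When the manager's click state is Settlement and the node is not yet settled, it disables click events, clears the state and asks the manager to build there.
; setPlayer records the owner and swaps the sphere material to that player's colour.
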(event `self.ReceiveBeginPlay`
  (bind _returnvalue (`GameplayStatics.GetActorOfClass` "/Game/BluePrints/BP_gameManager.BP_gameManager_C"))
  (set `self.gameManager` _returnvalue))

(event `setPlayer`
  (params (Player :type "/Game/BluePrints/BP_player Object Reference"))
  (`self.setVisualColour` Player))

(event `self.Sphere.OnClicked`
  (params (TouchedComponent :type "PrimitiveComponent Object Reference") (ButtonPressed :type "Key Structure"))
  (`self.settlementClickFunction` :!label _label))

(event `Debug Clicked(Sphere)`
  (goto _label))

(fn `settlementClickFunction`
  (bind _gamemanager (`self.gameManager`))
  (bind _gamemanager_2 (`self.gameManager`))
  (switch `/Game/Data/E_clickState` (`/Game/BluePrints/BP_gameManager.clickState` _gamemanager)
    (:`NewEnumerator0`
      (if (not (`KismetArrayLibrary.Array_Contains` (`/Game/BluePrints/BP_gameManager.settledNodes` _gamemanager) self))
        (set `PlayerController.bEnableClickEvents` false (`GameplayStatics.GetPlayerController` 0))
        (set `/Game/BluePrints/BP_gameManager.clickState` "NewEnumerator3" _gamemanager_2)
        (`/Game/BluePrints/BP_gameManager.buildSettlement` _gamemanager_2 self)))))

(fn `setVisualColour`
  (params (Player :type "/Game/BluePrints/BP_player Object Reference"))
  (bind _sphere (`self.Sphere`))
  (set `self.player` Player)
  (bind _output_get (set `self.colour` (`/Game/BluePrints/BP_player.colour` Player)))
  (switch `/Game/Data/E_playerColours` _output_get
    (:`NewEnumerator0`
      (`PrimitiveComponent.SetMaterial` _sphere 0 "/Game/Materials/M_baseRed.M_baseRed"))
    (:`NewEnumerator1`
      (`PrimitiveComponent.SetMaterial` _sphere 0 "/Game/Materials/M_baseBlue.M_baseBlue"))
    (:`NewEnumerator2`
      (`PrimitiveComponent.SetMaterial` _sphere 0 "/Game/Materials/M_baseGreen.M_baseGreen"))
    (:`NewEnumerator3`
      (`PrimitiveComponent.SetMaterial` _sphere 0 "/Game/Materials/M_baseYellow.M_baseYellow"))))

(fn `UserConstructionScript`)