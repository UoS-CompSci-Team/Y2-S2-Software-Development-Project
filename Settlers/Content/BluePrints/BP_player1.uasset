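; BP_player1 holds one player's state for a resource-building board game: score, resource hand, settlements and roads.
; Helper functions add victory points, edit the hand's resource-to-count map and append board pieces, though AddRoad has no node input wired.
; CheckBuild compares a cost map against the hand, stopping at the first shortfall.
; Debug strings report changes; BeginPlay is empty and the EventGraph's CheckBuild test is disconnected.
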(event `self.ReceiveBeginPlay`)

(fn `addResource`
  (params (resource :type "/Game/Data/E_resourceType Enum" :default "NewEnumerator0") (addNum :type Integer))
  (bind _hand_resourcecards (break `/Game/Data/S_playerHand` (`self.hand`)))
  ;[1 1 1] updates player hand and prints string
  (`BlueprintMapLibrary.Map_Add` _hand_resourcecards resource (+ (`BlueprintMapLibrary.Map_Find` _hand_resourcecards resource) addNum))
  (`KismetSystemLibrary.PrintString` "item added" true true (struct :`G` 0.66 :`B` 1.0 :`A` 1.0) 5.0))

(fn `addRoad`
  ;[1 1 1] adds board node (road) to player array
  (`KismetArrayLibrary.Array_Add` (`self.roads`)))

(fn `addSettlement`
  (params (settlementNode :type "/Game/BluePrints/BP_settlementNode Object Reference"))
  ;[1 1 1] adds board node (settlement) to player array
  (`KismetArrayLibrary.Array_Add` (`self.settlements`) settlementNode))

(fn `checkBuild`
  (params (settlement :type "Map of /Game/Data/E_resourceType Enum to Integer"))
  (returns (canBuild :type Boolean))
  (bind _hand_resourcecards (break `/Game/Data/S_playerHand` (`self.hand`)))
  ;[1 1 1] for each key value do...
  (bind _keys (`BlueprintMapLibrary.Map_Keys` settlement))
  (for _array_element _keys
    ;[1 1 1] if player does not have resource set "can build" var to false and break
    (if (not (>= (`BlueprintMapLibrary.Map_Find` _hand_resourcecards _array_element) (`BlueprintMapLibrary.Map_Find` settlement _array_element)))
      (bind _output_get (set `self.canBuild` false))
      (return _output_get)))
  ;[1 1 1] return "can build" after for each loop
  (return (`self.canBuild`)))

(fn `displayPlayerItems`
  (bind _hand_resourcecards (break `/Game/Data/S_playerHand` (`self.hand`)))
  ;[1 1 1] gets keys and for each value do...
  (bind _keys (`BlueprintMapLibrary.Map_Keys` _hand_resourcecards))
  (for _array_element _keys
    ;[1 1 1] print key
    (`KismetSystemLibrary.PrintString` (`KismetStringLibrary.Conv_IntToString` (`BlueprintMapLibrary.Map_Find` _hand_resourcecards _array_element)) true true (struct :`G` 0.66 :`B` 1.0 :`A` 1.0) 10.0)
    ;[1 1 1] prints keys
    (`KismetSystemLibrary.PrintString` (`|GetEnumeratorNameAsString` _array_element) true true (struct :`G` 0.66 :`B` 1.0 :`A` 1.0) 10.0)))

(fn `plusVictoryPoints`
  (params (numPoints :type Integer))
  (bind _returnvalue (+ numPoints (`self.score`)))
  ;[1 1 1] adds input number of victory points to player score
  (set `self.score` _returnvalue)
  (`KismetSystemLibrary.PrintString` (`KismetStringLibrary.Conv_IntToString` _returnvalue) true true (struct :`R` 1.0 :`G` 0.050922 :`B` 0.031026 :`A` 1.0) 10.0))

(fn `removeResource`
  (params (resource :type "/Game/Data/E_resourceType Enum" :default "NewEnumerator0") (removeNum :type Integer))
  (bind _hand_resourcecards (break `/Game/Data/S_playerHand` (`self.hand`)))
  ;[1 1 1] updates player hand and prints string
  (`BlueprintMapLibrary.Map_Add` _hand_resourcecards resource (- (`BlueprintMapLibrary.Map_Find` _hand_resourcecards resource) removeNum))
  (`KismetSystemLibrary.PrintString` "item has been removed" true true (struct :`G` 0.66 :`B` 1.0 :`A` 1.0) 5.0 "Nonec"))

(fn `UserConstructionScript`)