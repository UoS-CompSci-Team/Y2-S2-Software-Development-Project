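; Player Blueprint for a settlement-and-road board game, with logic to compute a player's longest road.
; FindDisjointRoads walks owned roads from settlements using a stack to build connected node sets; boardUpdate runs only this step.
; FindTerminalNodes picks single-road nodes from each set, or the first node if none exist.
; FindLongestRoad runs a recursive backtracking DFS from those starts, using a visited-node set, and keeps the maximum length.
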(event `boardUpdate`
  (`self.findDisjointRoads` null))

(fn `findDisjointRoads`
  (params (player :type "/Game/BluePrints/BP_player Object Reference"))
  (returns (settlementNodeSets :type "Array of /Game/Data/S_nodeSet Structure"))
  (locals (stack :type "Array of /Game/BluePrints/BP_settlementNode Object Reference") (roadSets :type "Array of /Game/Data/S_nodeSet Structure") (startNode :type "Array of /Game/BluePrints/BP_settlementNode Object Reference") (node :type "/Game/BluePrints/BP_settlementNode Object Reference") (nextNode :type "/Game/BluePrints/BP_settlementNode Object Reference") (foundSet :type Boolean))
  (bind _stack (`local.stack`))
  (bind _returnvalue (`KismetArrayLibrary.Array_LastIndex` _stack))
  (for _array_element (`/Game/BluePrints/BP_player.settlements` player)
    (`KismetArrayLibrary.Array_Add` _stack _array_element) ; add settlement to stack
    (while (`KismetArrayLibrary.Array_IsNotEmpty` _stack)
      ;[1 1 1] Pop last element into node
      (bind _output_get (set `local.node` (`|GetArrayItem` _stack _returnvalue)))
      (`KismetArrayLibrary.Array_Remove` _stack _returnvalue)
      (for _array_element_2 (`/Game/BluePrints/BP_settlementNode.roads` _output_get)
        (if (== (`/Game/BluePrints/BP_road.player` _array_element_2) (`local.player`))
          (bind _othernode (`/Game/BluePrints/BP_road.getOtherNode` _array_element_2 (`local.node`)))
          (`KismetArrayLibrary.Array_Add` (`local.stack`) _othernode) ; add nextNode to stack
          (for _array_element_3 (`local.roadSets`)
            (if (`BlueprintSetLibrary.Set_Contains` (break `/Game/Data/S_nodeSet` _array_element_3) (`local.node`))
              (set `local.foundSet` true) ; record that set has been found
              (`BlueprintSetLibrary.Set_Add` (break `/Game/Data/S_nodeSet` _array_element_3) (`local.nextNode`)) ; add next node to found set
              (break)))
          (if (not (`local.foundSet`))
            (`KismetArrayLibrary.Array_Add` (`local.roadSets`) (make `/Game/Data/S_nodeSet` (`|MakeSet` (`local.node`) (`local.nextNode`)))) ; add new set to roadSets
          )
          (return (`local.roadSets`)))))))

(fn `findLongestRoad`
  (params (player :type "/Game/BluePrints/BP_player Object Reference"))
  (returns (longestRoadLength :type Integer))
  (locals (result :type Integer))
  (bind _settlementnodesets (`self.findDisjointRoads` player))
  (bind _terminalnodes (`self.findTerminalNodes` _settlementnodesets))
  (for _array_element _terminalnodes
    (bind _result (`BlueprintSetLibrary.Set_ToArray` (break `/Game/Data/S_nodeSet` _array_element)))
    (for _array_element_2 _result
      (bind _finallength (`self.longestRoadDFS` (`local.player`) (`|MakeSet` null :!type "/Game/BluePrints/BP_settlementNode Object Reference") _array_element_2))
      (set `local.result` (`KismetMathLibrary.Max` _finallength (`local.result`)))))
  (return (`local.result`)))

(fn `findTerminalNodes`
  (params (disjointRoads :type "Array of /Game/Data/S_nodeSet Structure"))
  (returns (terminalNodes :type "Array of /Game/Data/S_nodeSet Structure"))
  (locals (res :type "Array of /Game/Data/S_nodeSet Structure") (temp :type "/Game/Data/S_nodeSet Structure"))
  (bind _res (`local.res`))
  (bind _temp_data (break `/Game/Data/S_nodeSet` (`local.temp`)))
  (bind _temp_data_2 (break `/Game/Data/S_nodeSet` (`local.temp`)))
  (for _array_element disjointRoads
    (set `local.temp` (make `/Game/Data/S_nodeSet` (`|MakeSet` null :!type "/Game/BluePrints/BP_settlementNode Object Reference"))) ; empty the temp set
    (bind _result (`BlueprintSetLibrary.Set_ToArray` (break `/Game/Data/S_nodeSet` _array_element)))
    (for _array_element_2 _result
      (if (== (`KismetArrayLibrary.Array_Length` (`/Game/BluePrints/BP_settlementNode.roads` _array_element_2)) 1)
        (`BlueprintSetLibrary.Set_Add` _temp_data _array_element_2)))
    ;[1 1 1] add tempData to res if tempData not empty else create set from first node and add to res
    (if (`BlueprintSetLibrary.Set_IsNotEmpty` _temp_data_2)
      (`KismetArrayLibrary.Array_Add` _res (`local.temp`))
      (else
        (`KismetArrayLibrary.Array_Add` _res (make `/Game/Data/S_nodeSet` (`|MakeSet` (`|GetArrayItem` _result)))))))
  (return (`local.res`)))

(fn `longestRoadDFS`
  (params (player :type "/Game/BluePrints/BP_player Object Reference") (visited :type "Set of /Game/BluePrints/BP_settlementNode Object Reference") (start :type "/Game/BluePrints/BP_settlementNode Object Reference") (length :type Integer))
  (returns (finalLength :type Integer))
  (locals (result :type Integer))
  (if (`BlueprintSetLibrary.Set_Contains` visited start)
    (return (`local.result`))
    (else
      (`BlueprintSetLibrary.Set_Add` (`local.visited`) (`local.start`))
      (set `local.result` (`local.length`))
      (for _array_element (`/Game/BluePrints/BP_settlementNode.roads` (`local.start`))
        (if (== (`/Game/BluePrints/BP_road.player` _array_element) (`local.player`))
          (bind _othernode (`/Game/BluePrints/BP_road.getOtherNode` _array_element (`local.start`)))
          (bind _finallength (`self.longestRoadDFS` (`local.player`) (`local.visited`) _othernode (+ (`local.length`) 1))) ; recursive
          (set `local.result` (`KismetMathLibrary.Max` (`local.result`) _finallength))))
      (`BlueprintSetLibrary.Set_Remove` (`local.visited`))
      (return (`local.result`)))))

(fn `UserConstructionScript`)