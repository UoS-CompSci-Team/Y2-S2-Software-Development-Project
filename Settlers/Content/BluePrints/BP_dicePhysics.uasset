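; BP_dicePhysics is a physics die actor that throws itself when play begins.
; BeginPlay gives the Cube a velocity-change impulse with randomized horizontal and upward strength, applied at a randomly offset point above its location so the off-center hit can add spin.
; Tick checks whether the Cube's linear velocity is exactly zero, but that branch does nothing, so no roll result is read.
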(event `self.ReceiveBeginPlay`
  (bind _cube (`self.Cube`))
  (bind (_returnvalue_x _returnvalue_y _returnvalue_z) (`KismetMathLibrary.BreakVector` (`SceneComponent.K2_GetComponentLocation` _cube)))
  (`PrimitiveComponent.AddVelocityChangeImpulseAtLocation` _cube (`KismetMathLibrary.MakeVector` (`KismetMathLibrary.Conv_IntToDouble` (`KismetMathLibrary.RandomIntegerInRange` 200 800)) (`KismetMathLibrary.Conv_IntToDouble` (`KismetMathLibrary.RandomIntegerInRange` 200 800)) (`KismetMathLibrary.Conv_IntToDouble` (`KismetMathLibrary.RandomIntegerInRange` 300 1000))) (`KismetMathLibrary.MakeVector` (+ _returnvalue_x (`KismetMathLibrary.RandomIntegerInRange` -30 30)) (+ _returnvalue_y (`KismetMathLibrary.RandomIntegerInRange` -30 30)) (+ _returnvalue_z (`KismetMathLibrary.RandomIntegerInRange` 20 80))) "None"))

(event `self.ReceiveTick`
  (params (DeltaSeconds :type "Float (single-precision)"))
  (bind _returnvalue (`PrimitiveComponent.GetPhysicsLinearVelocity` (`self.Cube`) "None"))
  (if (== _returnvalue (0.0 0.0 0.0))
    (if true
      _)))

(fn `UserConstructionScript`)