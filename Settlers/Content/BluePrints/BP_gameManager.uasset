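; BP_gameManager runs a four-player Catan-style board game, from randomised board setup to dice rolls, building and turn order.
; On BeginPlay it caches board actors, assigns hex resources and numbers, then creates the UI and players.
; A GameState machine toggles click events, while setup snake turns reverse the player array each round.
; Rolls pay settlements and cities on matching hexes, skipping the robber's; a seven starts robber placement.
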(event `self.ReceiveBeginPlay`
  ;[1 1 1] Game initialisation
  (add `self.gameStateUpdate` (delegate `gameStateUpdate_Event`))
  (`self.gameInitialisation`))

(event `gameStateUpdate_Event`
  ;[1 1 1] Game initialisation
  (`self.gameStateUpdate_Process`))

(event `Debug Roll Dice`
  (params (`Dice Roll` :type Integer))
  (bind _returnvalue (+ (`/Game/BluePrints/BP_die.lastRoll` (`self.dice1`)) (`/Game/BluePrints/BP_die.lastRoll` (`self.dice2`))))
  ;[0.01656 1 0] DEBUG: forced dice roll result
  (set `/Game/BluePrints/BP_die.lastRoll` `Dice Roll` (`self.dice1`))
  (set `/Game/BluePrints/BP_die.lastRoll` 0 (`self.dice2`))
  ;[1 1 1] When dice are rolled
  (`KismetSystemLibrary.PrintString` (`KismetStringLibrary.Conv_IntToString` _returnvalue) true true (struct :`G` 0.66 :`B` 1.0 :`A` 1.0) 10.0 :!label _label)
  (`self.playerPlaceRobberOn7` _returnvalue)
  (`self.giveDiceRollResourcesAlpha` _returnvalue))

(event `Debug Make Settlements Clickable`
  (`self.Change Game State` "NewEnumerator15"))

(event `/Game/Interfaces/I_UI_Interface.rollDice`
  ;[1 1 1] When dice are rolled
  (goto _label))

(event `/Game/Interfaces/I_UI_Interface.endTurn`
  ;[1 1 1] When next turn is called
  (`self.setNextPlayerToCurrentPlayer`)
  ;[1 1 1] If true still in set up phase
  (if (> (`self.snakeTurnsIndex`) 0)
    (`self.Change Game State` "NewEnumerator15")
    (else
      (set `self.developmentCardPurchased` false)
      (`self.Change Game State` "NewEnumerator9"))))

(event `buildSettlement`
  (params (Settlement :type "/Game/BluePrints/BP_settlementNode Object Reference"))
  (bind _currentplayer (`self.currentPlayer`))
  ;[1 1 1] When a settlement is built
  (`/Game/BluePrints/BP_player.storeSettlement` _currentplayer Settlement)
  (`/Game/BluePrints/BP_settlementNode.setPlayer` Settlement _currentplayer)
  (for _array_element (`/Game/BluePrints/BP_settlementNode.hexRefs` Settlement)
    (`/Game/BluePrints/BP_hexGrid.addSettlement` _array_element Settlement))
  (`self.whenSettlementIsSettledFunction` Settlement)
  (bind _returnvalue (`self.inSetupPhase`))
  (if _returnvalue
    (if (== (`self.snakeTurnsIndex`) 1)
      (`self.giveSecondSettlementResources` Settlement))
    (`self.playerPlaceRoad` true)
    (else
      (`/Game/BluePrints/BP_player.removeResource` _currentplayer (`self.settlementCost`)))))

(event `/Game/Interfaces/I_UI_Interface.buildSettlementCallFromUI`
  (`self.Change Game State` "NewEnumerator15"))

(event `/Game/Interfaces/I_UI_Interface.buildRoadCallFromUI`
  (bind _returnvalue (`self.inSetupPhase`))
  (`self.playerPlaceRoad` _returnvalue))

(event `/Game/Interfaces/I_UI_Interface.buildCityCallFromUI`
  (`self.playerUpgradeToCity`))

(event `Change Game State`
  (params (newGameState :type "/Game/Data/E_gameState Enum" :default "NewEnumerator27"))
  ;[1 1 1] game state functions
  (set `self.gameState` newGameState)
  (`self.gameStateUpdate`))

(event `gameStateUpdate_Process`
  (bind _returnvalue (`GameplayStatics.GetPlayerController` 0))
  ;[1 1 1] game state functions
  (switch `/Game/Data/E_gameState` (`self.gameState`)
    (:`NewEnumerator27`
      (set `PlayerController.bEnableClickEvents` false _returnvalue :!label _label_2))
    (:`NewEnumerator9`
      (goto _label_2))
    (:`NewEnumerator10`
      (goto _label_2))
    (:`NewEnumerator15`
      (set `PlayerController.bEnableClickEvents` true _returnvalue :!label _label_3))
    (:`NewEnumerator16`
      (goto _label_3))
    (:`NewEnumerator17`
      (goto _label_3))
    (:`NewEnumerator18`
      (goto _label_2))
    (:`NewEnumerator19`
      (goto _label_2))
    (:`NewEnumerator20`
      (goto _label_3))
    (:`NewEnumerator21`
      (goto _label_3))
    (:`NewEnumerator22`
      (goto _label_2))
    (:`NewEnumerator23`
      (goto _label_2))
    (:`NewEnumerator24`
      (goto _label_2))
    (:`NewEnumerator28`
      (goto _label_2))))

(event `Change Development Card Purchased`
  (params (newValue :type Boolean))
  ;[1 1 1] update development card (ready for event calling in the future)
  (set `self.developmentCardPurchased` newValue))

(fn `assignSettlementToPlayer`)

(fn `checkSettlementAvailablilty`
  ;[1 1 1] Is it assigned to a player?
  (for _array_element (`self.settlementsNodes`)
    (if (not (`KismetArrayLibrary.Array_Contains` (`self.settledNodes`) _array_element))
      ;[1 1 1] Enable click to build
      (`self.Change Game State` "NewEnumerator15"))))

(fn `createUI`
  (bind _returnvalue (`|CreateWidget` "/Game/UserInterface/W_PrototypeUI.W_PrototypeUI_C"))
  (bind _output_get (set `self.protoUI` _returnvalue))
  (`UserWidget.AddToViewport` _output_get 0)
  (set `/Game/UserInterface/W_PrototypeUI.gameManagerInstance` self _output_get)
  (`/Game/UserInterface/W_PrototypeUI.Initialise Widget` _output_get))

(fn `debugAllocateRandomSettlements`
  (locals (maxNumOfSettlements :type Integer :default 2) (`function Settlements` :type "Array of /Game/BluePrints/BP_settlementNode Object Reference"))
  (bind _function_settlements (`local.function Settlements`))
  (bind _output (`|GetArrayItem` _function_settlements))
  ;[1 1 1] Creates a copy of the settlement array and randomizes
  (bind _output_get (set `local.function Settlements` (`self.settlementsNodes`)))
  (`KismetArrayLibrary.Array_Shuffle` _output_get)
  ;[1 1 1] Sets a maximum number of settlements per player - so allocation cannot exceed the total amount of settlements
  (set `local.maxNumOfSettlements` 2)
  (for _array_element (`self.players`)
    (for _ (range 1 (+ (`local.maxNumOfSettlements`) 1))
      ;[1 1 1] Inner loop body
      (`/Game/BluePrints/BP_player.storeSettlement` _array_element _output)
      (`SceneComponent.SetVisibility` (`/Game/BluePrints/BP_settlementNode.Sphere` _output) true false)
      (`KismetArrayLibrary.Array_Remove` _function_settlements))))

(fn `gameInitialisation`
  (set `PlayerController.bShowMouseCursor` true (`GameplayStatics.GetPlayerController` 0))
  (`self.setRobberReference`)
  (`self.setHexGridResources`)
  (`self.setSettlementNodeArray`)
  (`self.setRoadsArray`)
  (`self.createUI`)
  (`self.setDiceReferences`)
  (`self.spawnPlayers`)
  (`self.checkSettlementAvailablilty`)
  (`self.Change Game State` "NewEnumerator15"))

(fn `giveDiceRollResources`
  (params (diceRoll :type Integer))
  (locals (add1 :type Integer) (add2 :type Integer))
  (for _array_element (`self.players`)
    (for _array_element_2 (`/Game/BluePrints/BP_player.settlements` _array_element)
      ;[1 1 1] For each hex - check if the associated hex dice no == rolled dice no
      (for _array_element_3 (`/Game/BluePrints/BP_settlementNode.hexRefs` _array_element_2)
        ;[1 1 1] Check if robber is on current hex
        (if (not (== _array_element_3 (`/Game/BluePrints/BP_robber.currentLocation` (`self.robber`))))
          ;[1 1 1] Gives resources to player - if settlement is a city = 2 x resources
          (if (== diceRoll (`/Game/BluePrints/BP_hexGrid.tileNumber` _array_element_3))
            (if (`/Game/BluePrints/BP_settlementNode.isCity?` _array_element_2)
              (bind _resourcetype (`/Game/BluePrints/BP_hexGrid.resourceType` _array_element_3))
              (`/Game/BluePrints/BP_player.addResource` _array_element _resourcetype 2)
              (else
                (`/Game/BluePrints/BP_player.addResource` _array_element _resourcetype 1)))))))))

(fn `giveDiceRollResourcesAlpha`
  (params (diceRoll :type Integer))
  (locals (add1 :type Integer) (add2 :type Integer) (tempResourceMap :type "Map of /Game/Data/E_resourceType Enum to Object Object Reference"))
  (bind _tempresourcemap (`local.tempResourceMap`))
  (bind _tempresourcemap_2 (`local.tempResourceMap`))
  (for _array_element (`self.players`)
    (set `local.tempResourceMap` (`|MakeMap` "NewEnumerator0" 0 "NewEnumerator1" 0 "NewEnumerator2" 0 "NewEnumerator4" 0 "NewEnumerator5" :!type "/Game/Data/E_resourceType Enum"))
    (for _array_element_2 (`/Game/BluePrints/BP_player.settlements` _array_element)
      ;[1 1 1] For each hex - check if the associated hex dice no == rolled dice no
      (for _array_element_3 (`/Game/BluePrints/BP_settlementNode.hexRefs` _array_element_2)
        (if (== diceRoll (`/Game/BluePrints/BP_hexGrid.tileNumber` _array_element_3))
          ;[1 1 1] Check if robber is on current hex
          (if (not (== _array_element_3 (`/Game/BluePrints/BP_robber.currentLocation` (`self.robber`))))
            ;[1 1 1] Gives resources to player - if settlement is a city = 2 x resources
            (if (`/Game/BluePrints/BP_settlementNode.isCity?` _array_element_2)
              (bind _resourcetype (`/Game/BluePrints/BP_hexGrid.resourceType` _array_element_3))
              (`BlueprintMapLibrary.Map_Add` _tempresourcemap _resourcetype (+ (`BlueprintMapLibrary.Map_Find` _tempresourcemap _resourcetype) 2))
              (else
                (`BlueprintMapLibrary.Map_Add` _tempresourcemap _resourcetype (+ (`BlueprintMapLibrary.Map_Find` _tempresourcemap _resourcetype) 1)))))))
      (`/Game/BluePrints/BP_player.addResourcesAlpha` _array_element _tempresourcemap_2)
      (`BlueprintMapLibrary.Map_Clear` _tempresourcemap_2))))

(fn `giveSecondSettlementResources`
  (params (settlement :type "/Game/BluePrints/BP_settlementNode Object Reference"))
  (locals (add1 :type Integer :default 1) (resourceToAdd :type "Map of /Game/Data/E_resourceType Enum to Object Object Reference"))
  (for _array_element (`/Game/BluePrints/BP_settlementNode.hexRefs` settlement)
    (bind _resourcetype (`/Game/BluePrints/BP_hexGrid.resourceType` _array_element))
    (`/Game/BluePrints/BP_player.addResource` (`self.currentPlayer`) _resourcetype 1)
    (`KismetSystemLibrary.PrintString` (`|GetEnumeratorNameAsString` _resourcetype))))

(fn `inSetupPhase`
  (returns (ReturnValue :type Boolean))
  (return (> (`self.snakeTurnsIndex`) 0)))

(fn `pickRandomCard`
  (params (cardStruct :type "/Game/Data/S_Hand Structure") (`isResource?` :type Boolean))
  (returns (ResourceCard :type "/Game/Data/E_resourceType Enum") (SpecialCard :type "/Game/Data/E_specialType Enum"))
  (locals (resourceToPickFrom :type "Array of /Game/Data/E_resourceType Enum") (victoryToPickFrom :type "Array of /Game/Data/E_specialType Enum"))
  (bind (_resourcecards _specialcards) (break `/Game/Data/S_Hand` cardStruct))
  (bind _resourcetopickfrom (`local.resourceToPickFrom`))
  (if `isResource?`
    (bind _keys (`BlueprintMapLibrary.Map_Keys` _resourcecards))
    ;[1 1 1] For each resource type, iterate through quantity and store in an array
    (for _array_element _keys
      (for _ (range (`BlueprintMapLibrary.Map_Find` _resourcecards _array_element))
        (`KismetArrayLibrary.Array_Add` (`local.resourceToPickFrom`) _array_element)))
    ;[1 1 1] if no cards in hand return None resource type - otherwise picks randomly
    (if (> (`KismetArrayLibrary.Array_Length` _resourcetopickfrom) 0)
      ;[1 1 1] return the resource card (ignore special card)
      (return (`KismetArrayLibrary.Array_Random` _resourcetopickfrom) "NewEnumerator0")
      (else
        (return "NewEnumerator7" "NewEnumerator0")))
    (else
      (bind _keys_2 (`BlueprintMapLibrary.Map_Keys` _specialcards))
      ;[1 1 1] For each special card, iterate through quantity and store in an array
      (for _array_element_2 _keys_2
        (for _ (range (`BlueprintMapLibrary.Map_Find` _specialcards _array_element_2))
          (`KismetArrayLibrary.Array_Add` (`local.victoryToPickFrom`) _array_element_2)))
      ;[1 1 1] return special card (ignore resource)
      (return "NewEnumerator0" (`KismetArrayLibrary.Array_Random` (`local.victoryToPickFrom`))))))

(fn `playerPlaceRoad`
  (params (isSetup :type Boolean))
  (bind _currentplayer (`self.currentPlayer`))
  (bind _settlements (`/Game/BluePrints/BP_player.settlements` _currentplayer))
  (if isSetup
    ;[1 1 1] Get adjacent roads to last placed settlement for setup phase
    (set `self.clickStateSelectableRoads` (`/Game/BluePrints/BP_settlementNode.adjacentRoads` (`|GetArrayItem` _settlements (`KismetArrayLibrary.Array_LastIndex` _settlements))))
    (else
      ;[1 1 1] Gets all roads that player can place when in normal play
      (for _array_element (`self.roads`)
        (bind _canbuild (`/Game/BluePrints/BP_road.canPlayerBuildRoad` _array_element _currentplayer))
        (if _canbuild
          (`KismetArrayLibrary.Array_Add` (`self.clickStateSelectableRoads`) _array_element)))))
  ;[1 1 1] For each of the selectable roads - makes them visible and binds the on click event
  (for _array_element_2 (`self.clickStateSelectableRoads`)
    (`SceneComponent.SetVisibility` (`/Game/BluePrints/BP_road.Plane` _array_element_2) true false)
    (add `self.OnClicked` _array_element_2 (`|CreateDelegate` :!event `Road on Click`)))
  ;[1 1 1] Enables click events
  (`self.Change Game State` "NewEnumerator17"))

(fn `playerPlaceRobberOn7`
  (params (DiceRoll :type Integer))
  (if (== DiceRoll 7)
    (`self.Change Game State` "NewEnumerator20")))

(fn `playerPlaceSettlement`
  ;[1 1 1] Does not fire if in snake turns
  (if (not (> (`self.snakeTurnsIndex`) 0))
    ;[0 1 0.001571] Removes from player the resource cards for settlement
    (`/Game/BluePrints/BP_player.removeResource` (`self.currentPlayer`) (`self.settlementCost`))
    ;[1 1 1] starts settlement pick process
    (`self.checkSettlementAvailablilty`)))

(fn `playerUpgradeToCity`
  (locals (upgradableSettlements :type "Array of /Game/BluePrints/BP_settlementNode Object Reference"))
  ;[1 1 1] Does not fire if in snake turns
  (if (not (> (`self.snakeTurnsIndex`) 0))
    ;[1 1 1] Sets the players settlements to a visibly clickable state
    (for _array_element (`/Game/BluePrints/BP_player.settlements` (`self.currentPlayer`))
      (if (not (`/Game/BluePrints/BP_settlementNode.isCity?` _array_element))
        (`KismetArrayLibrary.Array_Add` (`local.upgradableSettlements`) _array_element)
        (`PrimitiveComponent.SetRenderCustomDepth` (`/Game/BluePrints/BP_settlementNode.Sphere` _array_element) true)))
    ;[1 1 1] If there is 1+ upgradable settlments then click events are enabled
    (if (> (`KismetArrayLibrary.Array_Length` (`local.upgradableSettlements`)) 0)
      (`self.Change Game State` "NewEnumerator16"))))

(fn `Road on Click`
  (params (TouchedActor :type "Actor Object Reference") (ButtonPressed :type "Key Structure" :default "None"))
  (bind _clickstateselectableroads (`self.clickStateSelectableRoads`))
  (bind _currentplayer (`self.currentPlayer`))
  ;[0 1 0.1165] Click state check. Turn off click events and set click state to none. Changed for bug Fix: can't click on already built road
  (switch `/Game/Data/E_gameState` (`self.gameState`)
    (:`NewEnumerator17`
      (bind _asbp_road (cast `/Game/BluePrints/BP_road` TouchedActor))
      (bind _isbuiltupon (`/Game/BluePrints/BP_road.isBuiltUpon` _asbp_road))
      (if (not _isbuiltupon)
        (bind _returnvalue (`self.inSetupPhase`))
        (if _returnvalue
          (`self.Change Game State` "NewEnumerator27")
          (else
            (`self.Change Game State` "NewEnumerator10")))
        ;[1 1 1] Check the clicked road is in the array clickStateSelectableRoads
        (if (`KismetArrayLibrary.Array_Contains` _clickstateselectableroads _asbp_road)
          ;[1 1 1] removes the clicked road from selectableRoads and sets all roads that were selectable to invisible
          (`KismetArrayLibrary.Array_RemoveItem` _clickstateselectableroads _asbp_road)
          ;[1 1 1] Assign current player to the road piece and adds road to player array
          (`/Game/BluePrints/BP_road.setVisualColour` _asbp_road _currentplayer)
          (`/Game/BluePrints/BP_player.storeRoad` _currentplayer _asbp_road)
          (bind _returnvalue_2 (`self.inSetupPhase`))
          (if (not _returnvalue_2)
            (`/Game/BluePrints/BP_player.removeResource` _currentplayer (`self.roadCost`)))
          ;[1 1 1] Clear the selectable roads
          (`KismetArrayLibrary.Array_Clear` (`self.clickStateSelectableRoads`)))))))

(fn `setDiceReferences`
  (bind _protoui (`self.protoUI`))
  (bind _outactors (`GameplayStatics.GetAllActorsOfClass` "/Game/BluePrints/BP_die.BP_die_C"))
  (bind _output_get (set `self.dice1` (`|GetArrayItem` _outactors)))
  (set `/Game/UserInterface/W_PrototypeUI.dice1Instance` _output_get _protoui)
  (bind _output_get_2 (set `self.dice2` (`|GetArrayItem` _outactors 1)))
  (set `/Game/UserInterface/W_PrototypeUI.dice2Instance` _output_get_2 _protoui))

(fn `setHexGridResources`
  (locals (hexCopy :type "Array of /Game/BluePrints/BP_hexGrid Object Reference") (hexTemp :type "Array of /Game/BluePrints/BP_hexGrid Object Reference") (hexT :type "/Game/BluePrints/BP_hexGrid Object Reference") (hexNumberArray :type "Array of Integer") (passNum :type Integer) (selectedNum :type Integer) (selectedNumberIdx :type Integer))
  (bind _hexcopy (`local.hexCopy`))
  (bind _hexnumberarray (`local.hexNumberArray`))
  (bind _hexcopy_2 (`local.hexCopy`))
  (bind _hexcopy_3 (`local.hexCopy`))
  (bind _hexcopy_4 (`local.hexCopy`))
  (bind _hexcopy_5 (`local.hexCopy`))
  ;[1 1 1] Creat temp hex grid refs
  (for _array_element (`self.hexes`)
    (`KismetArrayLibrary.Array_Add` (`local.hexCopy`) _array_element))
  ;[1 1 1] Set desert tile
  (bind _output_get (set `local.hexT` (`|GetArrayItem` (`local.hexCopy`) (`KismetMathLibrary.RandomIntegerInRange` 0 18))))
  (set `/Game/BluePrints/BP_hexGrid.resourceType` "NewEnumerator6" _output_get)
  (`/Game/BluePrints/BP_hexGrid.setResource` _output_get)
  (`/Game/BluePrints/BP_robber.setToDesert` (`self.robber`) _output_get)
  (`KismetArrayLibrary.Array_RemoveItem` (`local.hexCopy`) _output_get)
  ;[1 1 1] Set 4 lumber tiles
  (for _ (range 4)
    (bind _output_get_2 (set `local.hexT` (`|GetArrayItem` _hexcopy (`KismetMathLibrary.RandomIntegerInRange` 0 (- (`KismetArrayLibrary.Array_Length` _hexcopy) 1)))))
    (`KismetArrayLibrary.Array_Add` (`local.hexTemp`) _output_get_2)
    (`KismetArrayLibrary.Array_RemoveItem` (`local.hexCopy`) _output_get_2))
  (for _array_element_2 (`local.hexTemp`)
    (set `/Game/BluePrints/BP_hexGrid.resourceType` "NewEnumerator4" _array_element_2)
    (`/Game/BluePrints/BP_hexGrid.setResource` _array_element_2))
  (`KismetArrayLibrary.Array_Clear` (`local.hexTemp`))
  ;[1 1 1] Set 4 grain tiles
  (for _ (range 4)
    (bind _output_get_3 (set `local.hexT` (`|GetArrayItem` _hexcopy_2 (`KismetMathLibrary.RandomIntegerInRange` 0 (- (`KismetArrayLibrary.Array_Length` _hexcopy_2) 1)))))
    (`KismetArrayLibrary.Array_Add` (`local.hexTemp`) _output_get_3)
    (`KismetArrayLibrary.Array_RemoveItem` (`local.hexCopy`) _output_get_3))
  (for _array_element_3 (`local.hexTemp`)
    (set `/Game/BluePrints/BP_hexGrid.resourceType` "NewEnumerator1" _array_element_3)
    (`/Game/BluePrints/BP_hexGrid.setResource` _array_element_3))
  (`KismetArrayLibrary.Array_Clear` (`local.hexTemp`))
  ;[1 1 1] Set 4 wool tiles
  (for _ (range 4)
    (bind _output_get_4 (set `local.hexT` (`|GetArrayItem` _hexcopy_3 (`KismetMathLibrary.RandomIntegerInRange` 0 (- (`KismetArrayLibrary.Array_Length` _hexcopy_3) 1)))))
    (`KismetArrayLibrary.Array_Add` (`local.hexTemp`) _output_get_4)
    (`KismetArrayLibrary.Array_RemoveItem` (`local.hexCopy`) _output_get_4))
  (for _array_element_4 (`local.hexTemp`)
    (set `/Game/BluePrints/BP_hexGrid.resourceType` "NewEnumerator2" _array_element_4)
    (`/Game/BluePrints/BP_hexGrid.setResource` _array_element_4))
  (`KismetArrayLibrary.Array_Clear` (`local.hexTemp`))
  ;[1 1 1] Set 3 ore tiles
  (for _ (range 3)
    (bind _output_get_5 (set `local.hexT` (`|GetArrayItem` _hexcopy_4 (`KismetMathLibrary.RandomIntegerInRange` 0 (- (`KismetArrayLibrary.Array_Length` _hexcopy_4) 1)))))
    (`KismetArrayLibrary.Array_Add` (`local.hexTemp`) _output_get_5)
    (`KismetArrayLibrary.Array_RemoveItem` (`local.hexCopy`) _output_get_5))
  (for _array_element_5 (`local.hexTemp`)
    (set `/Game/BluePrints/BP_hexGrid.resourceType` "NewEnumerator5" _array_element_5)
    (`/Game/BluePrints/BP_hexGrid.setResource` _array_element_5))
  (`KismetArrayLibrary.Array_Clear` (`local.hexTemp`))
  ;[1 1 1] Set 3 brick tiles
  (for _ (range 3)
    (bind _output_get_6 (set `local.hexT` (`|GetArrayItem` _hexcopy_5 (`KismetMathLibrary.RandomIntegerInRange` 0 (- (`KismetArrayLibrary.Array_Length` _hexcopy_5) 1)))))
    (`KismetArrayLibrary.Array_Add` (`local.hexTemp`) _output_get_6)
    (`KismetArrayLibrary.Array_RemoveItem` (`local.hexCopy`) _output_get_6))
  (for _array_element_6 (`local.hexTemp`)
    (set `/Game/BluePrints/BP_hexGrid.resourceType` "NewEnumerator0" _array_element_6)
    (`/Game/BluePrints/BP_hexGrid.setResource` _array_element_6))
  (`KismetArrayLibrary.Array_Clear` (`local.hexTemp`))
  ;[1 1 1] distribute numbers proportionately onto hex tiles (excluding desert)
  (for _array_element_7 (`self.hexes`)
    (if (`|EnumInequality` (`/Game/BluePrints/BP_hexGrid.resourceType` _array_element_7) "NewEnumerator6")
      (bind _output_get_7 (set `local.selectedNumberIdx` (`.OutIndex` (`KismetArrayLibrary.Array_Random` (`local.hexNumberArray`)))))
      (set `local.selectedNum` (`|GetArrayItem` _hexnumberarray _output_get_7))
      (`KismetArrayLibrary.Array_Remove` _hexnumberarray (`local.selectedNumberIdx`))
      (`/Game/BluePrints/BP_hexGrid.setNumber` _array_element_7 (`local.selectedNum`)))))

(fn `setNextPlayerToCurrentPlayer`
  (bind _output_get (set `self.currentPlayerIndex` (mod (+ 1 (`self.currentPlayerIndex`)) (`KismetArrayLibrary.Array_Length` (`self.players`)))))
  ;[1 1 1] Reverses the array for the snake style turn logic
  (if (and (> (`self.snakeTurnsIndex`) 0) (== 0 _output_get))
    (`KismetArrayLibrary.Array_Reverse` (`self.players`))
    (set `self.snakeTurnsIndex` (- (`self.snakeTurnsIndex`) 1)))
  (bind _output (`|GetArrayItem` (`self.players`) _output_get))
  (`KismetSystemLibrary.PrintString` (`KismetSystemLibrary.GetDisplayName` _output) true true (struct :`R` 0.173859 :`G` 1.0 :`B` 0.338172 :`A` 1.0))
  (set `self.currentPlayer` _output))

(fn `setRoadsArray`
  (bind _outactors (`GameplayStatics.GetAllActorsOfClass` "/Game/BluePrints/BP_road.BP_road_C"))
  (for _array_element _outactors
    (`KismetArrayLibrary.Array_Add` (`self.roads`) _array_element)))

(fn `setRobberReference`
  (bind _returnvalue (`GameplayStatics.GetActorOfClass` "/Game/BluePrints/BP_robber.BP_robber_C"))
  (set `self.robber` _returnvalue))

(fn `setSettlementNodeArray`
  (bind _outactors (`GameplayStatics.GetAllActorsOfClass` "/Game/BluePrints/BP_settlementNode.BP_settlementNode_C"))
  (for _array_element _outactors
    (`KismetArrayLibrary.Array_Add` (`self.settlementsNodes`) _array_element)))

(fn `spawnPlayers`
  (locals (targetLocation :type "Vector Structure"))
  ;[1 1 1] Get location to spawn player actors
  (bind _outactors (`GameplayStatics.GetAllActorsOfClass` "/Script/Engine.TargetPoint"))
  (set `local.targetLocation` (`self.K2_GetActorLocation` (`|GetArrayItem` _outactors)))
  (for _index (range 4)
    (bind _returnvalue (`|SpawnActorFromClass` "/Game/BluePrints/BP_player.BP_player_C" (`KismetMathLibrary.MakeTransform` (`local.targetLocation`)) "Undefined" "OverrideRootScale" null null))
    (`KismetArrayLibrary.Array_Add` (`self.players`) _returnvalue)
    (set `/Game/BluePrints/BP_player.name` (`KismetStringLibrary.Conv_IntToString` _index) _returnvalue)
    (switch `int` _index
      (:`0`
        (set `/Game/BluePrints/BP_player.colour` "NewEnumerator0" _returnvalue))
      (:`1`
        (set `/Game/BluePrints/BP_player.colour` "NewEnumerator1" _returnvalue))
      (:`2`
        (set `/Game/BluePrints/BP_player.colour` "NewEnumerator2" _returnvalue))
      (:`3`
        (set `/Game/BluePrints/BP_player.colour` "NewEnumerator3" _returnvalue))))
  (set `self.currentPlayerIndex` 0)
  ;[1 1 1] Set to 0 just for prototype
  (set `self.snakeTurnsIndex` 2)
  (set `self.currentPlayer` (`|GetArrayItem` (`self.players`))))

(fn `UserConstructionScript`
  (bind _outactors (`GameplayStatics.GetAllActorsOfClass` "/Game/BluePrints/BP_hexGrid.BP_hexGrid_C"))
  (set `self.hexes` _outactors))

(fn `whenSettlementIsSettledFunction`
  (params (Settlement :type "/Game/BluePrints/BP_settlementNode Object Reference"))
  ;[1 1 1] Add settlement and it's adjascents to list of settled nodes
  (`KismetArrayLibrary.Array_Add` (`self.settledNodes`) Settlement)
  (for _array_element (`/Game/BluePrints/BP_settlementNode.adjacentRoads` Settlement)
    (if (`KismetStringLibrary.EqualEqual_StrStr` (`KismetSystemLibrary.GetDisplayName` (`/Game/BluePrints/BP_road.nodeA` _array_element)) (`KismetSystemLibrary.GetDisplayName` Settlement))
      (`KismetArrayLibrary.Array_Add` (`self.settledNodes`) (`/Game/BluePrints/BP_road.nodeB` _array_element))
      (else
        (`KismetArrayLibrary.Array_Add` (`self.settledNodes`) (`/Game/BluePrints/BP_road.nodeA` _array_element))))))