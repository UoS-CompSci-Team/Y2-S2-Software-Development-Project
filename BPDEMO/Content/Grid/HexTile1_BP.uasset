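; Hex grid tile Blueprint that shows a random number from 2 to 12 on its Number text at BeginPlay.
; A Redo event loops back to reroll when the check draws 7, but the stored Num comes from a separate roll, so it can still be 7.
; When a BP_TopDownCharacter overlaps its Box, it prints that character's Health and the tile's Num.
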(event `self.ReceiveBeginPlay`
  (bind _returnvalue (`KismetMathLibrary.RandomIntegerInRange` 2 12))
  (if (!= _returnvalue 7) :!label _label
    (bind _output_get (set `self.num` _returnvalue))
    (`TextRenderComponent.K2_SetText` (`self.Number`) (`KismetTextLibrary.Conv_IntToText` _output_get))
    (else
      (`self.redo`))))

(event `redo`
  (goto _label))

(event `self.Box.OnComponentBeginOverlap`
  (params (OverlappedComponent :type "PrimitiveComponent Object Reference") (OtherActor :type "Actor Object Reference") (OtherComp :type "PrimitiveComponent Object Reference") (OtherBodyIndex :type Integer) (bFromSweep :type Boolean) (SweepResult :type "HitResult Structure (by ref)"))
  (bind _asbp_top_down_character (cast `/Game/TopDown/Blueprints/BP_TopDownCharacter` OtherActor))
  (`KismetSystemLibrary.PrintString` (`KismetStringLibrary.Conv_IntToString` (`/Game/TopDown/Blueprints/BP_TopDownCharacter.Health` _asbp_top_down_character)) true true (struct :`G` 0.66 :`B` 1.0 :`A` 1.0) 10.0)
  (`KismetSystemLibrary.PrintString` (`KismetStringLibrary.Conv_IntToString` (`self.num`)) true true (struct :`G` 0.66 :`B` 1.0 :`A` 1.0) 10.0))

(fn `UserConstructionScript`)